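; BP_ImFine is an effect actor that shows a dome, floor outline and inner plane, then fades out and destroys itself.
; Start reveals the meshes and drives their dynamic material opacities through chained increase and decrease timelines, then activates the sparkle effect.
; End runs the fade timeline before destroying the actor; BeginPlay currently auto-runs Start and End, eight seconds apart, as removable test code.
; The construction script multiplies each mesh's relative scale by its own variable.
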(event Custom|Start
  (bind _ns_sparkle (Variables|Default|GetNS_Sparkle))
  (Rendering|SetVisibility (Variables|Default|GetSM_Plane_Inner) true false)
  (Rendering|SetVisibility (Variables|Default|GetSM_Outline) true false)
  (Rendering|SetVisibility (Variables|Default|GetSM_Dome) true false)
  (bind (_direction _sphere _outline _opacity) (Timeline|TL_IncreaseAmount PlayFromStart)
    (:Update
      (Rendering|Material|SetScalarParameterValue (Variables|Default|GetMI_Sphere) "Opacity" _sphere :!class /Script/Engine.MaterialInstanceDynamic)
      (Rendering|Material|SetScalarParameterValue (Variables|Default|GetMI_OutLine) "Opacity" _outline :!class /Script/Engine.MaterialInstanceDynamic)
      (Rendering|Material|SetScalarParameterValue (Variables|Default|GetMI_Inner) "Opacity" _opacity :!class /Script/Engine.MaterialInstanceDynamic))
    (:Finished
      (bind _sphere_2 (Timeline|TL_DecreaseAmount PlayFromStart)
        (:Update
          (Rendering|Material|SetScalarParameterValue (Variables|Default|GetMI_Sphere) "Opacity" _sphere_2 :!class /Script/Engine.MaterialInstanceDynamic))
        (:Finished
          (Rendering|SetVisibility _ns_sparkle true false)
          (Components|Activation|SetActive _ns_sparkle true false))))))

(event Custom|End
  (bind (_direction _opacity _sphere_opacity) (Timeline|TL_End PlayFromStart)
    (:Update
      (Rendering|Material|SetScalarParameterValue (Variables|Default|GetMI_Inner) "Opacity" _opacity :!class /Script/Engine.MaterialInstanceDynamic)
      (Rendering|Material|SetScalarParameterValue (Variables|Default|GetMI_OutLine) "Opacity" _opacity :!class /Script/Engine.MaterialInstanceDynamic)
      (Rendering|Material|SetScalarParameterValue (Variables|Default|GetMI_Sphere) "Genaral_Opacity" _sphere_opacity :!class /Script/Engine.MaterialInstanceDynamic))
    (:Finished
      (Actor|DestroyActor))))

(event EventBeginPlay
  (bind _returnvalue (Rendering|Material|CreateDynamicMaterialInstance (Variables|Default|GetSM_Dome) 0 0 "None" :!class /Script/Engine.PrimitiveComponent))
  (Variables|Default|SetMI_Sphere _returnvalue)
  (bind _returnvalue_2 (Rendering|Material|CreateDynamicMaterialInstance (Variables|Default|GetSM_Outline) 0 0 "None" :!class /Script/Engine.PrimitiveComponent))
  (Variables|Default|SetMI_OutLine _returnvalue_2)
  (bind _returnvalue_3 (Rendering|Material|CreateDynamicMaterialInstance (Variables|Default|GetSM_Plane_Inner) 0 0 "None" :!class /Script/Engine.PrimitiveComponent))
  (Variables|Default|SetMI_Inner _returnvalue_3)
  ;[0 0 0] TestCode (삭제해도 됨)
  (CallFunction|Start)
  (Utilities|FlowControl|Delay 8.0)
  (CallFunction|End))

(fn ConstructionScript
  (CallFunction|SetScales))

(fn SetScales
  (bind _sm_plane_inner (Variables|Default|GetSM_Plane_Inner))
  (bind _sm_outline (Variables|Default|GetSM_Outline))
  (bind _sm_dome (Variables|Default|GetSM_Dome))
  (Transformation|SetRelativeScale3D _sm_dome (* (Variables|/Script/Engine.SceneComponent|GetRelativeScale3D _sm_dome) (Variables|Default|GetSM_Dome_ScaleMultiply)))
  (Transformation|SetRelativeScale3D _sm_outline (* (Variables|/Script/Engine.SceneComponent|GetRelativeScale3D _sm_outline) (Variables|Default|GetSM_Floor_Outline_ScaleMultiply)))
  (Transformation|SetRelativeScale3D _sm_plane_inner (* (Variables|/Script/Engine.SceneComponent|GetRelativeScale3D _sm_plane_inner) (Variables|Default|GetSM_Plane_Inner_ScaleMultiply))))