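; Base ranged-attack projectile Blueprint with configurable colors for its body, tail and impact effect.
; On BeginPlay it creates a dynamic material instance for the mesh and applies the projectile color to it and the tail color to the Niagara trail.
; On any collision overlap it spawns a tinted Niagara impact at its own location, using the other actor's rotation, then destroys itself.
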(event OnComponentBeginOverlap(Collision)
  (params (OverlappedComponent :type Primitive%20Component%20Object%20Reference) (OtherActor :type Actor%20Object%20Reference) (OtherComp :type Primitive%20Component%20Object%20Reference) (OtherBodyIndex :type Integer) (bFromSweep :type Boolean) (SweepResult :type Hit%20Result%20Structure%20%28by%20ref%29))
  ;[0 0 0] 히트 될 때 이펙트 스폰
  (bind _returnvalue (Niagara|SpawnSystematLocation "/Game/FX/BaseRangedAttack/NS_BaseProjectile_Imapact.NS_BaseProjectile_Imapact" (Transformation|GetActorLocation) (Transformation|GetActorRotation OtherActor)))
  ;;[0 0 0] 히트 될 때, 스폰되는 이펙트 색 조정
  (Effects|Components|ParticleSystem|SetColorParameter _returnvalue "Impact_Color" (Variables|Default|GetImpactColor))
  (Actor|DestroyActor))

(event EventBeginPlay
  (bind _returnvalue (Rendering|Material|CreateDynamicMaterialInstance "/Game/FX/BaseRangedAttack/MI_BaseProjectile.MI_BaseProjectile" "None" "None" :!class /Script/Engine.KismetMaterialLibrary))
  (Variables|Default|SetMI_Projectile%20Material _returnvalue)
  (Rendering|Material|SetMaterial (Variables|Default|GetStaticMesh_Projectile) 0 _returnvalue)
  ;[0 0 0] 컬러 조정
  ;;[0 0 0] 투사체 컬러
  (Rendering|Material|SetVectorParameterValue (Variables|Default|GetMI_Projectile%20Material) "Color" (Variables|Default|GetProjectileColor) :!class /Script/Engine.MaterialInstanceDynamic)
  ;;[0 0 0] 꼬리 컬러
  (Effects|Components|ParticleSystem|SetColorParameter (Variables|Default|GetNiagara_Tail) "TailColor" (Variables|Default|GetTailColor)))

(fn ConstructionScript)