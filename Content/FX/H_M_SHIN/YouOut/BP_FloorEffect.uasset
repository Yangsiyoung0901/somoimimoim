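; BP_FloorEffect is a floor visual effect for YouOut, staged through Hit1, Hit2 and Hit3 events.
; Hit1 hides and deactivates the NSYouOutImpact effect and grows Ring1, while Hit2 grows Ring2.
; Both rings scale up in X and Y on fast looping timers that clear themselves past a size limit.
; Hit3 collapses both rings, resets their scale counters and shows and activates the impact effect.
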(event Custom|Hit1
  (bind _returnvalue (Utilities|Time|SetTimerbyEvent (delegate Custom|Event_Hit1) 0.01 true))
  (Variables|Default|SetTimer_Hit1 _returnvalue)
  (Rendering|SetVisibility (Variables|Default|GetNS_YouOut_Impact) false false)
  (Components|Activation|SetActive (Variables|Default|GetNS_YouOut_Impact) false false))

(event Custom|Hit2
  (bind _returnvalue (Utilities|Time|SetTimerbyEvent (delegate Custom|Event_Hit2) 0.01 true))
  (Variables|Default|SetTimer_Hit2 _returnvalue))

(event Custom|Event_Hit1
  (Transformation|SetRelativeScale3D (Variables|Default|GetRing1) (Math|Vector|MakeVector (Variables|Default|GetScale_Ring1) (Variables|Default|GetScale_Ring1) 1.0))
  (if (> (Variables|Default|GetScale_Ring1) 0.7)
    (Utilities|Time|ClearandInvalidateTimerbyHandle (Variables|Default|GetTimer_Hit1))
    (else
      (Variables|Default|SetScale_Ring1 (+ (Variables|Default|GetScale_Ring1) 0.07)))))

(event Custom|Event_Hit2
  (Transformation|SetRelativeScale3D (Variables|Default|GetRing2) (Math|Vector|MakeVector (Variables|Default|GetScale_Hit2) (Variables|Default|GetScale_Hit2) 1.0))
  (if (> (Variables|Default|GetScale_Hit2) 1.0)
    (Utilities|Time|ClearandInvalidateTimerbyHandle (Variables|Default|GetTimer_Hit2))
    (else
      (Variables|Default|SetScale_Hit2 (+ (Variables|Default|GetScale_Hit2) 0.1)))))

(event Custom|Hit3
  (Transformation|SetRelativeScale3D (Variables|Default|GetRing1) (Math|Vector|MakeVector 0.0 0.0 1.0))
  (Transformation|SetRelativeScale3D (Variables|Default|GetRing2) (Math|Vector|MakeVector 0.0 0.0 1.0))
  (Variables|Default|SetScale_Ring1 0.0)
  (Variables|Default|SetScale_Hit2 0.0)
  (Rendering|SetVisibility (Variables|Default|GetNS_YouOut_Impact) true false)
  (Components|Activation|SetActive (Variables|Default|GetNS_YouOut_Impact) true false))

(event EventBeginPlay)

(event Collision|EventActorBeginOverlap
  (params (OtherActor :type Actor%20Object%20Reference)))

(event EventTick
  (params (DeltaSeconds :type Float%20%28single-precision%29)))

(fn ConstructionScript)