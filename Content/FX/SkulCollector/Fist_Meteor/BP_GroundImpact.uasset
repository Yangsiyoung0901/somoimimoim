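; BP_GroundImpact is the ground impact effect for the Skul Collector's Fist Meteor, built around the NSGroundImpact particle component.
; The construction script multiplies one Scale variable by per-layer base values to set sizes, speeds and spawn radii.
; These parameters cover the floor effect, flare, big and small explosions, and sprite burst, so the effect resizes from a single value.
; The event graph holds only empty default events.
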(event EventBeginPlay)

(event Collision|EventActorBeginOverlap
  (params (OtherActor :type Actor%20Object%20Reference)))

(event EventTick
  (params (DeltaSeconds :type Float%20%28single-precision%29)))

(fn ConstructionScript
  (bind _ns_ground_impact (Variables|Default|GetNS_Ground_Impact))
  (bind _scale (Variables|Default|GetScale))
  (Utilities|FlowControl|Sequence
    (:then_0
      ;[0 0 0 1 30] 바닥 이펙트
      (Niagara|SetNiagaraVariable(Float) _ns_ground_impact "Size_Floor" (* _scale 1.4)))
    (:then_1
      ;[0 0 0 1 30] 플레어
      (Niagara|SetNiagaraVariable(Float) _ns_ground_impact "Size_Flare" (* _scale 3e+02)))
    (:then_2
      ;[0 0 0 1 30] 큰 폭발 이펙트
      (Niagara|SetNiagaraVariable(Float) _ns_ground_impact "Size_Big_Explosion" (* _scale 2e+02))
      (Niagara|SetNiagaraVariable(Float) _ns_ground_impact "Speed_Scale_Big_Explosion" (* _scale 1.0)))
    (:then_3
      ;[0 0 0 1 30] 작은 폭발 이펙트
      (Niagara|SetNiagaraVariable(Float) _ns_ground_impact "Size_Small_Explosion" (* _scale 1e+02))
      (Niagara|SetNiagaraVariable(Float) _ns_ground_impact "Size_SphereRadius_Small_Explosion" (* _scale 1e+01))
      (Niagara|SetNiagaraVariable(Float) _ns_ground_impact "Speed_Small_Explosion" (* _scale 4e+02)))
    (:then_4
      ;[0 0 0 1 30] 터지는 스프라이트 파티클
      (Class|NiagaraComponent|SetVariableVec2 _ns_ground_impact "Size_Min_Sprites_Burst" (* _scale "(X=0.100000,Y=3.000000)"))
      (Class|NiagaraComponent|SetVariableVec2 _ns_ground_impact "Size_Max_Sprites_Burst" (* _scale "(X=0.200000,Y=5.000000)"))
      (Niagara|SetNiagaraVariable(Float) _ns_ground_impact "Size_SphereRadius_Sprites_Burst" (* _scale 1.0))
      (Niagara|SetNiagaraVariable(Float) _ns_ground_impact "Speed_Min_Sprites_Burst" (* _scale 1e+02))
      (Niagara|SetNiagaraVariable(Float) _ns_ground_impact "Speed_Max_Sprites_Burst" (* _scale 4e+02)))))