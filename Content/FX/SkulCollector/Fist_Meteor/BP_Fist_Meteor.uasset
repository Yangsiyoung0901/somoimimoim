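; Fist meteor projectile effect that dives diagonally and bursts on the floor.
; A single Scale value drives the construction script, sizing the fist, setting projectile velocity and tuning the Spark trail's size and position parameters.
; BeginPlay offsets the fist up and back along that path by a scaled distance.
; Overlapping a Floor-tagged actor spawns a scaled BP_GroundImpact at world Z zero, activates its Niagara effect, then destroys the meteor after a short delay.
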(event OnComponentBeginOverlap(Sphere)
  (params (OverlappedComponent :type Primitive%20Component%20Object%20Reference) (OtherActor :type Actor%20Object%20Reference) (OtherComp :type Primitive%20Component%20Object%20Reference) (OtherBodyIndex :type Integer) (bFromSweep :type Boolean) (SweepResult :type Hit%20Result%20Structure%20%28by%20ref%29))
  (bind _returnvalue (Transformation|GetActorRotation))
  (bind _fist (Variables|Default|GetFist))
  (bind _returnvalue_2 (Transformation|GetWorldLocation _fist))
  (bind (_roll _pitch _yaw) (Math|Rotator|BreakRotator _returnvalue))
  (if (Actor|ActorHasTag OtherActor "Floor")
    (bind _returnvalue_3 (Game|SpawnActorfromClass "/Game/FX/SkulCollector/Fist_Meteor/BP_GroundImpact.BP_GroundImpact_C" (Math|Transform|MakeTransform (Math|Vector|MakeVector (.x _returnvalue_2) (.y _returnvalue_2) 0.0) (Math|Rotator|MakeRotator _roll _pitch (+ _yaw 9e+01)) "1.000000,1.000000,1.000000") "AlwaysSpawn" "MultiplyWithRoot" 0 (* (Variables|Default|GetScale) 2.0) 0))
    (Components|Activation|SetActive (Variables|/Game/FX/SkulCollector/Fist_Meteor/BP_GroundImpact.BP_GroundImpact_C|GetNS_Ground_Impact _returnvalue_3) true false)
    (Utilities|FlowControl|Delay 0.5)
    (Actor|DestroyActor)))

(event EventBeginPlay
  (bind _fist (Variables|Default|GetFist))
  (Transformation|SetRelativeLocation _fist (+ (Variables|/Script/Engine.SceneComponent|GetRelativeLocation _fist) (* (Variables|Default|GetScale) "-4000.000000,0.000000,4000.000000")) false false))

(fn ConstructionScript
  (bind _spark (Variables|Default|GetSpark))
  (bind _scale (Variables|Default|GetScale))
  (Utilities|FlowControl|Sequence
    (:then_0
      ;[0 0 0 1 30] 꼬리 이펙트 제외한 나머지 스케일
      (Transformation|SetRelativeScale3D (Variables|Default|GetFist) (Math|Conversions|ToVector(Float) _scale))
      (Variables|/Script/Engine.MovementComponent|SetVelocity (Variables|Default|GetProjectileMovement) (* (Variables|Default|GetScale) "4000.000000,0.000000,-4000.000000")))
    (:then_1
      ;[0 0 0 1 30] 꼬리 이펙트 스케일
      ;;[0 0 0 1 30] 꼬리 이펙트 컬러
      (Class|NiagaraComponent|SetVariableVec2 _spark "Size_Fire_Color_" (* _scale "(X=20.000000,Y=200.000000)")))
    (:then_2
      ;;[0 0 0 1 30] 꼬리 이펙트 그레이
      (Class|NiagaraComponent|SetVariableVec2 _spark "Size_Min_Fire_Gray" (* _scale "(X=50.000000,Y=200.000000)"))
      (Class|NiagaraComponent|SetVariableVec2 _spark "Size_Max_Fire_Gray" (* _scale "(X=200.000000,Y=400.000000)")))
    (:then_3
      ;;[0 0 0 1 30] 꼬리 이펙트 초기 위치
      (Niagara|SetNiagaraVariable(Vector3) _spark "Position" (* _scale "0.000000,0.000000,75.000000")))))