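; Visual effect actor for the Patissiere character's passive, combining a Niagara system with ring and shockwave meshes.
; On BeginPlay it spawns the Niagara system inactive and creates dynamic material instances for the Ring and OutWave components.
; Start activates the particles and plays an Opacity timeline that drives both materials' Opacity parameter.
; Kill deactivates the particles and reverses the timeline to fade the materials back.
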(event Custom|Start
  (Components|Activation|Activate (Variables|Default|GetNS_Passive) false)
  (bind _opacity (Timeline|Opacity PlayFromStart)
    (:Update
      (Rendering|Material|SetScalarParameterValue (Variables|Default|GetMI_Ring) "Opacity" _opacity :!class /Script/Engine.MaterialInstanceDynamic)
      (Rendering|Material|SetScalarParameterValue (Variables|Default|GetMI_ShockWave) "Opacity" _opacity :!class /Script/Engine.MaterialInstanceDynamic))))

(event Custom|Kill
  (Components|Activation|Deactivate (Variables|Default|GetNS_Passive))
  (bind _opacity (Timeline|Opacity ReverseFromEnd)
    (:Update
      (Rendering|Material|SetScalarParameterValue (Variables|Default|GetMI_Ring) "Opacity" _opacity :!class /Script/Engine.MaterialInstanceDynamic)
      (Rendering|Material|SetScalarParameterValue (Variables|Default|GetMI_ShockWave) "Opacity" _opacity :!class /Script/Engine.MaterialInstanceDynamic))))

(event EventBeginPlay
  (bind _returnvalue (Niagara|SpawnSystemAttached "/Game/FX/ThePatissiere/Passive/NS_Patissiere_Passive.NS_Patissiere_Passive" (Variables|Default|GetDefaultSceneRoot) "None" (Transformation|GetActorLocation) (Transformation|GetActorRotation) "KeepWorldPosition" false false))
  (Variables|Default|SetNS_Passive _returnvalue)
  (bind _returnvalue_2 (Rendering|Material|CreateDynamicMaterialInstance (Variables|Default|GetRing) 0 "/Game/FX/ThePatissiere/Passive/MI_BasicRing_Out.MI_BasicRing_Out" "None" :!class /Script/Engine.PrimitiveComponent))
  (Variables|Default|SetMI_Ring _returnvalue_2)
  (bind _returnvalue_3 (Rendering|Material|CreateDynamicMaterialInstance (Variables|Default|GetOutWave) 0 "/Game/FX/ThePatissiere/Passive/MI_ShockWave_OutWave.MI_ShockWave_OutWave" "None" :!class /Script/Engine.PrimitiveComponent))
  (Variables|Default|SetMI_ShockWave _returnvalue_3))

(event Collision|EventActorBeginOverlap
  (params (OtherActor :type Actor%20Object%20Reference)))

(event EventTick
  (params (DeltaSeconds :type Float%20%28single-precision%29)))

(fn ConstructionScript)