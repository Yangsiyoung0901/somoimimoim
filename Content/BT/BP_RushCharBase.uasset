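; BP_RushCharBase is a character base Blueprint with a rush skill that raises its move speed while it is far from its target.
; Tick checks the distance to TargetCharacter against a fixed threshold.
; Two DoOnce nodes reset each other, so TypeSkill_Rush fires only when the threshold is crossed, adding a fixed speed bonus when far and subtracting it when close.
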(event Custom|TypeSkill_Rush
  (params (On :type Boolean))
  (Variables|Default|SetMoveSpeed (+ (Variables|Default|GetMoveSpeed) (Math|Float|SelectFloat 2e+02 -2e+02 On))))

(event EventBeginPlay
  (|CallParentFunction) ; 지금 이 노드는 비활성 상태입니다. \n핀을 끌어서 다른 노드를 연결하면 활성화됩니다.
)

(event Collision|EventActorBeginOverlap
  (params (OtherActor :type Actor%20Object%20Reference))
  (|CallParentFunction OtherActor) ; 지금 이 노드는 비활성 상태입니다. \n핀을 끌어서 다른 노드를 연결하면 활성화됩니다.
)

(event EventTick
  (params (DeltaSeconds :type Float%20%28single-precision%29))
  (|CallParentFunction DeltaSeconds)
  (if (>= (CallFunction|GetDistancewithTarget (Variables|Default|GetTarget%20Character)) 4e+02)
    (Utilities|FlowControl|DoOnce false :!label _label
      (:Completed
        (CallFunction|TypeSkillRush true)
        (goto _label_2 Reset)))
    (else
      (Utilities|FlowControl|DoOnce false :!label _label_2
        (:Completed
          (CallFunction|TypeSkillRush false)
          (goto _label Reset))))))

(fn ConstructionScript
  (|CallParentFunction))