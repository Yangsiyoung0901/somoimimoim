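; Base Blueprint for a tank character that evaluates when its type skill is usable and performs a taunt.
; Every tick it adds living enemies within a fixed radius to the skill target list, removes those outside, and sets the skill condition when at least two remain.
; TauntPlay spawns a warrior shout effect and plays the taunt montage, calling TauntEnd when it blends out or is interrupted.
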(event Custom|TauntPlay
  (Niagara|SpawnSystematLocation "/Game/Marketplace/RPGEffects/ParticlesNiagara/Warrior/Shout/NS_Warrior_Shout.NS_Warrior_Shout" (Transformation|GetActorLocation) "0, 0, 0" "2.000000,2.000000,2.000000")
  (Animation|Montage|PlayMontage (Variables|Character|GetMesh) "/Game/Animation/Montage/Tank_Taunt.Tank_Taunt"
    (:OnBlendOut
      _)
    (:OnInterrupted
      _))
  (Default|CallTauntEnd))

(event EventBeginPlay
  (|CallParentFunction))

(event Collision|EventActorBeginOverlap
  (params (OtherActor :type Actor%20Object%20Reference))
  (|CallParentFunction OtherActor) ; 지금 이 노드는 비활성 상태입니다. \n핀을 끌어서 다른 노드를 연결하면 활성화됩니다.
)

(event EventTick
  (params (DeltaSeconds :type Float%20%28single-precision%29))
  (bind _typeskilltarget (Variables|Default|GetTypeSkillTarget))
  (|CallParentFunction DeltaSeconds)
  (for _array_element (CallFunction|GetAllAliveEnemy)
    (if (<= (CallFunction|GetDistancewithTarget _array_element) 6e+02)
      (Utilities|Array|AddUnique _typeskilltarget _array_element)
      (else
        (Utilities|Array|RemoveItem _typeskilltarget _array_element))))
  (Variables|Default|SetTypeSkillCondition (>= (Utilities|Array|Length (Variables|Default|GetTypeSkillTarget)) 2)))

(fn ConstructionScript
  (|CallParentFunction))