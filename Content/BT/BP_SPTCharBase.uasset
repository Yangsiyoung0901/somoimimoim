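; Base Blueprint for support (SPT) characters that heal teammates, damage enemies and push back attackers.
; BaseAttack heals a same-team target with a Niagara effect, giving any overheal to the caster, or deals normal damage otherwise.
; The server's Tick enables the type skill when GetNearestEnemy finds a nearby, eligible enemy targeting this character.
; TypeSkill applies brief CC and uses a timeline to shove that enemy toward a navmesh-projected point, unblocked during the push.
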(event Custom|TypeSkill
  (bind (_find _target) (CallFunction|GetNearestEnemy))
  (if _find
    (bind _output_get (Variables|Default|SetTypeSkillTarget _target))
    (Default|ApplyCC (Variables|/Game/BT/AICharacterBase.AICharacterBase_C|GetBPC_CCs _output_get) "NewEnumerator8" 0.5)
    (Transformation|SetActorRotation (Math|Conversions|RotationFromXVector (Math|Vector|Normalize (- (Transformation|GetActorLocation (Variables|Default|GetTypeSkillTarget)) (Transformation|GetActorLocation)))))
    (Variables|Default|SetPushLocation (.ProjectedLocation (AI|Navigation|ProjectPointtoNavigation (+ (Transformation|GetActorLocation (Variables|Default|GetTypeSkillTarget)) (* (Math|Vector|Normalize (- (Transformation|GetActorLocation (Variables|Default|GetTypeSkillTarget)) (Transformation|GetActorLocation))) 6e+02)) 0 0 "400.000000,400.000000,400.000000")))
    (Default|SetCharUnblocked (Variables|Default|GetTypeSkillTarget) true)
    (bind _새_트랙_0 (Timeline|타임라인 PlayFromStart)
      (:Update
        (Transformation|SetActorLocation (Variables|Default|GetTypeSkillTarget) (Math|Vector|Lerp(Vector) (Transformation|GetActorLocation (Variables|Default|GetTypeSkillTarget)) (Math|Vector|MakeVector (.x (Variables|Default|GetPushLocation)) (.y (Variables|Default|GetPushLocation)) (.Z (Math|Vector|BreakVector (Transformation|GetActorLocation (Variables|Default|GetTypeSkillTarget))))) _새_트랙_0) true false))
      (:Finished
        (Default|SetCharUnblocked (Variables|Default|GetTypeSkillTarget) false)))))

(event Custom|PlayHealEffect
  (params (Target :type AI%20Character%20Base%20Object%20Reference))
  (Niagara|SpawnSystemAttached "/Game/Marketplace/RPGEffects/ParticlesNiagara/Priest/HealOverTime/NS_Preist_Heal_Over_Time_3D.NS_Preist_Heal_Over_Time_3D" (Variables|/Script/Engine.Character|GetMesh Target) "None" "0, 0, 0" "0, 0, 0" "SnapToTargetIncludingScale" true))

(event EventBeginPlay
  (|CallParentFunction) ; 지금 이 노드는 비활성 상태입니다. \n핀을 끌어서 다른 노드를 연결하면 활성화됩니다.
)

(event Collision|EventActorBeginOverlap
  (params (OtherActor :type Actor%20Object%20Reference))
  (|CallParentFunction OtherActor) ; 지금 이 노드는 비활성 상태입니다. \n핀을 끌어서 다른 노드를 연결하면 활성화됩니다.
)

(event EventTick
  (params (DeltaSeconds :type Float%20%28single-precision%29))
  (|CallParentFunction DeltaSeconds)
  (if (Networking|IsServer)
    (bind _find (CallFunction|GetNearestEnemy))
    (if _find
      (Variables|Default|SetTypeSkillCondition true)
      (else
        (Variables|Default|SetTypeSkillCondition false)))))

(event EventBaseAttack
  (bind _attacktarget (Variables|Default|GetAttackTarget))
  (bind _healeffectbuff (Variables|Default|GetHealEffectBuff))
  (bind _buffedad (Variables|Default|GetBuffedAD))
  (bind _defaultad (Variables|Default|GetDefaultAD))
  (bind _additionalad (Variables|Default|GetAdditionalAD))
  (bind _losthp (Default|GetLostHP _attacktarget))
  (bind _returnvalue (* _buffedad 0.01))
  (bind _returnvalue_2 (+ _defaultad _additionalad))
  (bind _returnvalue_3 (+ _returnvalue 1.0))
  (bind _returnvalue_4 (* _returnvalue_2 _returnvalue_3 _healeffectbuff))
  (if (== (Variables|/Game/BT/AICharacterBase.AICharacterBase_C|GetTeam (Variables|Default|GetAttackTarget)) (Variables|Default|GetTeam))
    (if (> _returnvalue_4 _losthp)
      (CallFunction|HealCharacter (- _returnvalue_4 _losthp))
      (Default|HealCharacter (Variables|Default|GetAttackTarget) _returnvalue_4)
      (else
        (Default|HealCharacter _attacktarget _returnvalue_4)))
    (CallFunction|PlayHealEffect (Variables|Default|GetAttackTarget))
    (else
      (CallFunction|DealDamageNormal (Variables|Default|GetAttackTarget) 1.0 false false "BaseAttack"))))

(fn ConstructionScript
  (|CallParentFunction))

(fn GetNearestEnemy
  (LocalVariables|SetNearestDistance 8e+02)
  (for _array_element (CallFunction|GetAllAliveEnemy)
    (if (Math|Boolean|ANDBoolean (<= (Default|GetDistancewithTarget _array_element self) (LocalVariables|GetNearestDistance)) (not (Variables|/Game/BT/AICharacterBase.AICharacterBase_C|GetIsUnstoppable _array_element)) (not (Utilities|Array|ContainsItem (Variables|/Game/BT/AICharacterBase.AICharacterBase_C|GetCCs _array_element) "NewEnumerator8")) (== (Variables|/Game/BT/AICharacterBase.AICharacterBase_C|GetTarget%20Character _array_element) self) (Utilities|Enum|NotEqual(Enum) (Variables|/Game/BT/AICharacterBase.AICharacterBase_C|GetActType _array_element) "NewEnumerator2"))
      (LocalVariables|SetNearestEnemy _array_element)
      (LocalVariables|SetNearestDistance (Default|GetDistancewithTarget _array_element self))))
  (bind _nearestenemy (LocalVariables|GetNearestEnemy)
    (:then
      (return true _nearestenemy))
    (:else
      (return false 0))))