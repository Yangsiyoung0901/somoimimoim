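; Actor component that applies timed crowd-control effects, Taunt and Wound, to its owning AICharacterBase.
; ApplyCC routes to each effect, which updates the character's CCs list and sets a removal timer.
; Wound only refreshes when the new time is at least the remaining time, while Taunt always takes the new target and time.
; The owner's death clears all effects, and the taunt target's death removes Taunt.
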(event Custom|ApplyCC
  (params (CC :type E_CrowdControls%20Enum :default "NewEnumerator0") (Time :type Float%20%28double-precision%29) (Target :type AI%20Character%20Base%20Object%20Reference))
  (switch Utilities|FlowControl|Switch|SwitchonE_CrowdControls CC
    (:NewEnumerator2
      (CallFunction|Taunt Time Target))
    (:NewEnumerator4
      (CallFunction|Wound Time))))

(event Custom|Wound
  (params (Time :type Float%20%28double-precision%29))
  (if (Utilities|Time|IsValidTimerHandle (Variables|Default|GetWoundTimerHandle))
    (if (<= (Utilities|Time|GetTimerRemainingTimebyHandle (Variables|Default|GetWoundTimerHandle)) Time)
      (Utilities|Time|ClearandInvalidateTimerbyHandle (Variables|Default|GetWoundTimerHandle))
      (bind _returnvalue (Utilities|Time|SetTimerbyEvent (delegate Custom|RemoveWound) Time :!label _label))
      (Variables|Default|SetWoundTimerHandle _returnvalue))
    (else
      (Utilities|Array|AddUnique (Variables|/Game/BT/AICharacterBase.AICharacterBase_C|GetCCs (Variables|Default|GetCharacter)) "NewEnumerator4")
      (goto _label))))

(event Custom|RemoveWound
  (Utilities|Array|RemoveItem (Variables|/Game/BT/AICharacterBase.AICharacterBase_C|GetCCs (Variables|Default|GetCharacter)) "NewEnumerator4")
  (Utilities|Time|ClearandInvalidateTimerbyHandle (Variables|Default|GetWoundTimerHandle)))

(event Custom|Taunt
  (params (Time :type Float%20%28double-precision%29) (Target :type AI%20Character%20Base%20Object%20Reference))
  (bind _taunttimerhandle (Variables|Default|GetTauntTimerHandle))
  (if (Utilities|Time|IsValidTimerHandle _taunttimerhandle)
    (Utilities|Time|ClearandInvalidateTimerbyHandle _taunttimerhandle)
    (else
      (Utilities|Array|AddUnique (Variables|/Game/BT/AICharacterBase.AICharacterBase_C|GetCCs (Variables|Default|GetCharacter)) "NewEnumerator2")))
  (bind _output_get (Variables|Default|SetTauntTarget Target))
  (Utilities|Time|SetTimerbyEvent (delegate Custom|RemoveTaunt) Time)
  (EventDispatchers|AssignCharDead _output_get (delegate Custom|RemoveTaunt)))

(event Custom|RemoveTaunt
  (bind _taunttarget (Variables|Default|GetTauntTarget)
    (:then
      (EventDispatchers|UnbindEventfromCharDead _taunttarget (delegate Custom|RemoveTaunt))
      (Variables|Default|SetTauntTarget 0)
      (Utilities|Array|RemoveItem (Variables|/Game/BT/AICharacterBase.AICharacterBase_C|GetCCs (Variables|Default|GetCharacter)) "NewEnumerator2")
      (Utilities|Time|ClearandInvalidateTimerbyHandle (Variables|Default|GetTauntTimerHandle)))
    (:else)))

(event Custom|RemoveAllCCs
  (CallFunction|RemoveTaunt)
  (CallFunction|RemoveWound))

(event EventBeginPlay
  (bind _asaicharacter_base (Utilities|Casting|CastToAICharacterBase (Components|GetOwner)))
  (bind _output_get (Variables|Default|SetCharacter _asaicharacter_base))
  (EventDispatchers|AssignCharDead _output_get (delegate Custom|RemoveAllCCs)))

(event EventTick
  (params (DeltaSeconds :type Float%20%28single-precision%29)))