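; Actor component that manages timed crowd-control states (Stun, Taunt, Wound, Force Move) and immunity on an AICharacterBase owner.
; ApplyCC routes to per-effect events that update the character's CCs array and set removal timers, with Unstoppable blocking all but Wound.
; Reapplication keeps the longer duration, except Taunt, which always replaces it, toggles an effect and ends if its target dies.
; Owner death removes all four CCs.
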(event Custom|ApplyCC
  (params (CC :type E_CrowdControls%20Enum :default "NewEnumerator0") (Time :type Float%20%28double-precision%29) (Target :type AI%20Character%20Base%20Object%20Reference))
  (switch Utilities|FlowControl|Switch|SwitchonE_CrowdControls CC
    (:NewEnumerator0
      (CallFunction|Stun Time))
    (:NewEnumerator2
      (CallFunction|Taunt Time Target))
    (:NewEnumerator4
      (CallFunction|Wound Time))
    (:NewEnumerator8
      (CallFunction|ForceMove Time))))

(event Custom|ForceMove
  (params (Time :type Float%20%28double-precision%29))
  (if (not (Variables|/Game/BT/AICharacterBase.AICharacterBase_C|GetIsUnstoppable (Variables|Default|GetCharacter)))
    (if (Utilities|Time|IsValidTimerHandle (Variables|Default|GetForceMoveHandle))
      (if (<= (Utilities|Time|GetTimerRemainingTimebyHandle (Variables|Default|GetForceMoveHandle)) Time)
        (Utilities|Time|ClearandInvalidateTimerbyHandle (Variables|Default|GetForceMoveHandle))
        (bind _returnvalue (Utilities|Time|SetTimerbyEvent (delegate Custom|RemoveForceMove) Time :!label _label))
        (Variables|Default|SetForceMoveHandle _returnvalue)
        (Default|CallGetCC "NewEnumerator8"))
      (else
        (Utilities|Array|AddUnique (Variables|/Game/BT/AICharacterBase.AICharacterBase_C|GetCCs (Variables|Default|GetCharacter)) "NewEnumerator8")
        (goto _label)))))

(event Custom|RemoveWound
  (Utilities|Array|RemoveItem (Variables|/Game/BT/AICharacterBase.AICharacterBase_C|GetCCs (Variables|Default|GetCharacter)) "NewEnumerator4")
  (Utilities|Time|ClearandInvalidateTimerbyHandle (Variables|Default|GetWoundTimerHandle)))

(event Custom|Stun
  (params (Time :type Float%20%28double-precision%29))
  (if (not (Variables|/Game/BT/AICharacterBase.AICharacterBase_C|GetIsUnstoppable (Variables|Default|GetCharacter)))
    (if (Utilities|Time|IsValidTimerHandle (Variables|Default|GetStunHandle))
      (if (<= (Utilities|Time|GetTimerRemainingTimebyHandle (Variables|Default|GetStunHandle)) Time)
        (Utilities|Time|ClearandInvalidateTimerbyHandle (Variables|Default|GetStunHandle))
        (bind _returnvalue (Utilities|Time|SetTimerbyEvent (delegate Custom|RemoveStun) Time :!label _label))
        (Variables|Default|SetStunHandle _returnvalue)
        (Default|CallGetCC "NewEnumerator0"))
      (else
        (Utilities|Array|AddUnique (Variables|/Game/BT/AICharacterBase.AICharacterBase_C|GetCCs (Variables|Default|GetCharacter)) "NewEnumerator0")
        (goto _label)))))

(event Custom|RemoveStun
  (Utilities|Array|RemoveItem (Variables|/Game/BT/AICharacterBase.AICharacterBase_C|GetCCs (Variables|Default|GetCharacter)) "NewEnumerator0")
  (Utilities|Time|ClearandInvalidateTimerbyHandle (Variables|Default|GetStunHandle)))

(event Custom|PlayCCEffect
  (params (On :type Boolean) (CC :type E_CrowdControls%20Enum :default "NewEnumerator0"))
  (bind _character (Variables|Default|GetCharacter))
  (bind _taunteffect (Variables|/Game/BT/AICharacterBase.AICharacterBase_C|GetTauntEffect _character))
  (bind _returnvalue (Utilities|Select :Index CC :NewEnumerator0 0 :NewEnumerator1 0 :NewEnumerator2 _taunteffect :NewEnumerator3 0 :NewEnumerator4 0 :NewEnumerator5 0 :NewEnumerator6 0 :NewEnumerator7 0 :NewEnumerator8 0))
  (if On
    (Rendering|SetVisibility _returnvalue true false)
    (else
      (Rendering|SetVisibility _returnvalue false false))))

(event Custom|ImmuneTimer
  (Variables|Default|SetIsImmune false)
  (Utilities|Time|ClearandInvalidateTimerbyHandle (Variables|Default|GetImuneTimerHandle)))

(event Custom|Taunt
  (params (Time :type Float%20%28double-precision%29) (Target :type AI%20Character%20Base%20Object%20Reference))
  (if (not (Variables|/Game/BT/AICharacterBase.AICharacterBase_C|GetIsUnstoppable (Variables|Default|GetCharacter)))
    (if (Utilities|Time|IsValidTimerHandle (Variables|Default|GetTauntTimerHandle))
      (Utilities|Time|ClearandInvalidateTimerbyHandle (Variables|Default|GetTauntTimerHandle))
      (else
        (Utilities|Array|AddUnique (Variables|/Game/BT/AICharacterBase.AICharacterBase_C|GetCCs (Variables|Default|GetCharacter)) "NewEnumerator2")))
    (bind _output_get (Variables|Default|SetTauntTarget Target))
    (CallFunction|PlayCCEffect true "NewEnumerator2")
    (bind _returnvalue (Utilities|Time|SetTimerbyEvent (delegate Custom|RemoveTaunt) Time))
    (EventDispatchers|AssignCharDead _output_get (delegate Custom|커스텀이벤트))
    (Variables|Default|SetTauntTimerHandle _returnvalue)
    (Default|CallGetCC "NewEnumerator2")))

(event Custom|RemoveTaunt
  (CallFunction|PlayCCEffect false "NewEnumerator2")
  (bind _taunttarget (Variables|Default|GetTauntTarget)
    (:then
      (EventDispatchers|UnbindEventfromCharDead _taunttarget (delegate Custom|커스텀이벤트))
      (Variables|Default|SetTauntTarget 0))
    (:else
      _))
  (Utilities|Array|RemoveItem (Variables|/Game/BT/AICharacterBase.AICharacterBase_C|GetCCs (Variables|Default|GetCharacter)) "NewEnumerator2")
  (Utilities|Time|ClearandInvalidateTimerbyHandle (Variables|Default|GetTauntTimerHandle)))

(event Custom|ApplyImune
  (params (Time :type Float%20%28double-precision%29))
  (if (Utilities|Time|IsValidTimerHandle (Variables|Default|GetImuneTimerHandle))
    (if (<= (Utilities|Time|GetTimerRemainingTimebyHandle (Variables|Default|GetImuneTimerHandle)) Time)
      (Utilities|Time|ClearandInvalidateTimerbyHandle (Variables|Default|GetImuneTimerHandle))
      (bind _returnvalue (Utilities|Time|SetTimerbyEvent (delegate Custom|ImmuneTimer) Time :!label _label))
      (Variables|Default|SetImuneTimerHandle _returnvalue))
    (else
      (Variables|Default|SetIsImmune true)
      (goto _label))))

(event Custom|RemoveAllCCs
  (params (Character :type AI%20Character%20Base%20Object%20Reference))
  (CallFunction|RemoveTaunt)
  (CallFunction|RemoveWound)
  (CallFunction|RemoveStun)
  (CallFunction|RemoveForceMove))

(event Custom|RemoveForceMove
  (Utilities|Array|RemoveItem (Variables|/Game/BT/AICharacterBase.AICharacterBase_C|GetCCs (Variables|Default|GetCharacter)) "NewEnumerator8")
  (Utilities|Time|ClearandInvalidateTimerbyHandle (Variables|Default|GetForceMoveHandle)))

(event Custom|커스텀이벤트
  (params (Character :type AI%20Character%20Base%20Object%20Reference))
  (CallFunction|RemoveTaunt))

(event Custom|Wound
  (params (Time :type Float%20%28double-precision%29))
  (if (Utilities|Time|IsValidTimerHandle (Variables|Default|GetWoundTimerHandle))
    (if (<= (Utilities|Time|GetTimerRemainingTimebyHandle (Variables|Default|GetWoundTimerHandle)) Time)
      (Utilities|Time|ClearandInvalidateTimerbyHandle (Variables|Default|GetWoundTimerHandle))
      (bind _returnvalue (Utilities|Time|SetTimerbyEvent (delegate Custom|RemoveWound) Time :!label _label))
      (Variables|Default|SetWoundTimerHandle _returnvalue))
    (else
      (Utilities|Array|AddUnique (Variables|/Game/BT/AICharacterBase.AICharacterBase_C|GetCCs (Variables|Default|GetCharacter)) "NewEnumerator4")
      (goto _label))))

(event EventBeginPlay
  (bind _asaicharacter_base (Utilities|Casting|CastToAICharacterBase (Components|GetOwner)))
  (bind _output_get (Variables|Default|SetCharacter _asaicharacter_base))
  (EventDispatchers|AssignCharDead _output_get (delegate Custom|RemoveAllCCs)))

(event EventTick
  (params (DeltaSeconds :type Float%20%28single-precision%29)))