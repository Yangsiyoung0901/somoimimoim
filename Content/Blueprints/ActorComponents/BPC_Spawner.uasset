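; Actor component that respawns its owning AI character after death, handled on the server.
; BeginPlay caches the owner's class, level, team and starting transform and binds to its death event, which triggers a level-scaled delay for levels 2 to 5.
; During battle, unless IsSpawnInGame is set, Respawn spawns a replacement, retrying next tick on failure, then plays a Niagara effect and announces it.
; The old owner is destroyed either way.
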(event Custom|CharDead_이벤트
  (params (Character :type AI%20Character%20Base%20Object%20Reference))
  (if (Networking|IsServer)
    (switch int (Variables|Default|GetCharLevel)
      (:2
        (Utilities|FlowControl|Delay 3.0))
      (:3
        (Utilities|FlowControl|Delay 4.0))
      (:4
        (Utilities|FlowControl|Delay 6.0))
      (:5
        (Utilities|FlowControl|Delay 8.0)))
    (CallFunction|Respawn)))

(event Custom|Respawn
  (bind _inittransform (Variables|Default|GetInitTransform))
  (bind _assimul_test_gamemode (Utilities|Casting|CastToSimul_TestGamemode (Game|GetGameMode)))
  (if (and (Variables|/Game/Simul_TestGamemode.Simul_TestGamemode_C|GetInBattle _assimul_test_gamemode) (not (Variables|Default|GetIsSpawnInGame)))
    (bind _returnvalue (Game|SpawnActorfromClass (Variables|Default|GetCharClass) _inittransform "Undefined" "MultiplyWithRoot" 0 (Variables|Default|GetTeam) (Variables|Default|GetCharLevel) 0 :!label _label))
    (Utilities|IsValid _returnvalue
      (:Is%20Valid
        (CallFunction|SpawnEffect (.Location (Math|Transform|BreakTransform _inittransform)))
        (Default|CallCharRespawn _returnvalue)
        (Utilities|FlowControl|DelayUntilNextTick)
        (Actor|DestroyActor (Components|GetOwner)))
      (:Is%20Not%20Valid
        (Utilities|FlowControl|DelayUntilNextTick)
        (goto _label)))
    (else
      (Actor|DestroyActor (Components|GetOwner)))))

(event Custom|SpawnEffect
  (params (SpawnedCharLoc :type Vector))
  (Niagara|SpawnSystematLocation "/Game/FX/CommonFX/LevelUP/NS_LevelUp.NS_LevelUp" (+ SpawnedCharLoc "0.000000,0.000000,-60.000000")))

(event EventBeginPlay
  (if (Networking|IsServer)
    (bind _asaicharacter_base (Utilities|Casting|CastToAICharacterBase (Components|GetOwner)))
    (Variables|Default|SetCharClass (Utilities|GetClass _asaicharacter_base))
    (Variables|Default|SetCharLevel (Variables|/Game/BT/AICharacterBase.AICharacterBase_C|GetLevel _asaicharacter_base))
    (Variables|Default|SetInitTransform (Transformation|GetActorTransform _asaicharacter_base))
    (Variables|Default|SetTeam (Variables|/Game/BT/AICharacterBase.AICharacterBase_C|GetTeam _asaicharacter_base))
    (EventDispatchers|AssignCharDead _asaicharacter_base (delegate Custom|CharDead_이벤트))))

(event EventTick
  (params (DeltaSeconds :type Float%20%28single-precision%29)))