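; Patissiere support character that throws desserts at the ally or self with the most lost HP percentage, or the whole living team from level 5.
; From level 3, a server-side Tick check scales skill acceleration with nearby allies.
; From level 4, an ally danger-of-death callback clears own CCs and, once, holds that ally invulnerable at 1 HP.
; This arms the ultimate, which levels up (capped) and fully heals that ally.
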(event Custom|CallDangerOfDeath_이벤트
  (params (Character :type AI%20Character%20Base%20Object%20Reference))
  (if (not (Variables|Default|GetIsDead))
    (Default|RemoveAllCCs (Variables|Default|GetBPC_CCs))
    (Variables|Default|SetReviveCharacter Character)
    (Utilities|FlowControl|DoOnce false
      (:Completed
        (Variables|/Game/BT/AICharacterBase.AICharacterBase_C|SetCurrentHP (Variables|Default|GetReviveCharacter) 1.0)
        (Variables|/Game/BT/AICharacterBase.AICharacterBase_C|SetIgnoreDamage (Variables|Default|GetReviveCharacter) true)
        (Variables|Default|SetUltSkillCondition true)))))

(event Custom|UltEffect
  (Utilities|FlowControl|Delay 0.4)
  (Niagara|SpawnSystematLocation "/Game/FX/CommonFX/LevelUP/NS_LevelUp.NS_LevelUp" (Transformation|GetActorLocation (Variables|Default|GetReviveCharacter))))

(event EventBeginPlay
  (|CallParentFunction))

(event Collision|EventActorBeginOverlap
  (params (OtherActor :type Actor%20Object%20Reference))
  (|CallParentFunction OtherActor) ; 지금 이 노드는 비활성 상태입니다. \n핀을 끌어서 다른 노드를 연결하면 활성화됩니다.
)

(event EventTick
  (params (DeltaSeconds :type Float%20%28single-precision%29))
  (|CallParentFunction DeltaSeconds)
  (Utilities|FlowControl|Sequence
    (:then_0
      (if (and (Networking|IsServer) (Variables|Default|GetPassiveActivate))
        (bind _number (CallFunction|PassiveAllyNumber))
        (if (!= _number (Variables|Default|GetNowPassiveNumber))
          (Variables|Default|SetAdditionalSkillAcceleration (+ (Variables|Default|GetAdditionalSkillAcceleration) (* (- _number (Variables|Default|GetNowPassiveNumber)) 40)))
          (CallFunction|ApplyStatChange)
          (Variables|Default|SetNowPassiveNumber _number))))))

(event EventActiveSkill
  (bind _self self)
  (bind _self_2 self)
  (if (>= (Variables|Default|GetLevel) 5)
    (for _array_element (CallFunction|GetAllAliveTeams)
      (bind _returnvalue (Game|SpawnActorfromClass "/Game/Blueprints/Characters/ThePatissiere/BP_Patissiere_ActiveSkill.BP_Patissiere_ActiveSkill_C" (Math|Transform|MakeTransform (Transformation|GetActorLocation) "0, 0, 0" "1.000000,1.000000,1.000000") "Undefined" "MultiplyWithRoot" 0 _array_element _self (Variables|Default|GetLevel) _self 0))
      (Default|ThrowDessert _returnvalue))
    (else
      (bind _target (CallFunction|GetActiveSkillTarget))
      (bind _returnvalue_2 (Game|SpawnActorfromClass "/Game/Blueprints/Characters/ThePatissiere/BP_Patissiere_ActiveSkill.BP_Patissiere_ActiveSkill_C" (Math|Transform|MakeTransform (Transformation|GetActorLocation) "0, 0, 0" "1.000000,1.000000,1.000000") "Undefined" "MultiplyWithRoot" 0 _target _self_2 (Variables|Default|GetLevel) _self_2 0))
      (Default|ThrowDessert _returnvalue_2))))

(event EventUltSkill
  (bind _revivecharacter (Variables|Default|GetReviveCharacter))
  (bind _revivecharacter_2 (Variables|Default|GetReviveCharacter))
  (bind _level (Variables|/Game/BT/AICharacterBase.AICharacterBase_C|GetLevel _revivecharacter))
  (bind _returnvalue (+ _level 1))
  (Variables|Default|SetUltSkillCondition false)
  (CallFunction|UltEffect)
  (Utilities|FlowControl|Delay 0.4)
  (if (!= _returnvalue 6)
    (Default|LevelChange _revivecharacter _returnvalue))
  (Variables|/Game/BT/AICharacterBase.AICharacterBase_C|SetCurrentHP _revivecharacter_2 (Default|GetMaxHP _revivecharacter_2))
  (Variables|/Game/BT/AICharacterBase.AICharacterBase_C|SetIgnoreDamage _revivecharacter_2 false))

(event EventBattleStartServer
  (|CallParentFunction)
  (Utilities|FlowControl|Sequence
    (:then_0
      (Variables|Default|SetPassiveActivate (>= (Variables|Default|GetLevel) 3)))
    (:then_1
      (if (>= (Variables|Default|GetLevel) 4)
        (for _array_element (CallFunction|GetAllAliveAllies)
          (EventDispatchers|AssignCallDangerOfDeath _array_element (delegate Custom|CallDangerOfDeath_이벤트)))))))

(event EventLevelChange
  (params (Level :type Integer))
  (|CallParentFunction Level)
  (Utilities|FlowControl|Sequence
    (:then_0
      (Variables|Default|SetPassiveActivate (>= (Variables|Default|GetLevel) 3)))
    (:then_1
      (if (>= (Variables|Default|GetLevel) 4)
        (for _array_element (CallFunction|GetAllAliveAllies)
          (EventDispatchers|AssignCallDangerOfDeath _array_element (delegate Custom|CallDangerOfDeath_이벤트)))))))

(fn ConstructionScript
  (|CallParentFunction))

(fn GetAllAliveTeams
  (bind _output_get (LocalVariables|SetAlly (CallFunction|GetAllAliveAllies)))
  (Utilities|Array|Add _output_get self)
  (return (LocalVariables|GetAlly)))

(fn GetActiveSkillTarget
  (for _array_element (CallFunction|GetAllAliveTeams)
    (if (and (>= (.Percentage (Default|GetLostHP _array_element)) (LocalVariables|GetMaxLostHP)) (not (Variables|/Game/BT/AICharacterBase.AICharacterBase_C|GetHealBanned _array_element)))
      (LocalVariables|SetMaxLostHP (.Percentage (Default|GetLostHP _array_element)))
      (LocalVariables|SetHealTarget _array_element)))
  (return (LocalVariables|GetHealTarget)))

(fn PassiveAllyNumber
  (LocalVariables|SetNum 0)
  (for _array_element (CallFunction|GetAllAliveAllies)
    (if (<= (Default|GetDistancewithTarget _array_element self) 8e+02)
      (Math|Integer|IncrementInt (LocalVariables|GetNum))))
  (return (LocalVariables|GetNum)))