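; Projectile actor for the Patissiere's active skill: a randomly chosen dessert thrown at a target to heal and buff it.
; A timeline arcs it to the target with multicast location updates, then hides it and applies a lost-HP-based heal and an attack bonus.
; A looping timer adds heal ticks until count or death ends it.
; Level 5 also grants max HP, halved under a specific CC, and keeps the attack bonus.
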(event Custom|ThrowDessert
  (bind _character (Variables|Default|GetCharacter))
  (bind _target (Variables|Default|GetTarget))
  (bind _level (Variables|Default|GetLevel))
  (bind _target_2 (Variables|Default|GetTarget))
  (bind _target_3 (Variables|Default|GetTarget))
  (bind _losthp (Default|GetLostHP _target_2))
  (bind _returnvalue (* _level 0.01))
  (bind _healeffectbuff (Variables|/Game/BT/AICharacterBase.AICharacterBase_C|GetHealEffectBuff _character))
  (bind _returnvalue_2 (* _losthp _returnvalue))
  (bind _returnvalue_3 (+ _returnvalue_2 0.03))
  (bind _returnvalue_4 (* _returnvalue_3 _healeffectbuff))
  (Variables|Default|SetOriginLocation (Transformation|GetActorLocation))
  (bind (_direction _location _z) (Timeline|타임라인 PlayFromStart)
    (:Update
      (CallFunction|SetActorLocationMulticast (Math|Vector|MakeVector (.x (Math|Vector|Lerp(Vector) (Variables|Default|GetOriginLocation) (Transformation|GetActorLocation (Variables|Default|GetTarget)) _location)) (.y (Math|Vector|Lerp(Vector) (Variables|Default|GetOriginLocation) (Transformation|GetActorLocation (Variables|Default|GetTarget)) _location)) (+ (+ (* _z 2e+02) (* (Default|GetDistancewithTarget (Variables|Default|GetCharacter) (Variables|Default|GetTarget)) 0.5 _z)) (.Z (Math|Vector|BreakVector (Variables|Default|GetOriginLocation)))))))
    (:Finished
      (CallFunction|SetVisibleMulticast)
      (if (Variables|/Game/BT/AICharacterBase.AICharacterBase_C|GetIsDead (Variables|Default|GetTarget))
        (Actor|DestroyActor)
        (else
          (if (== (Variables|Default|GetLevel) 5)
            (Variables|/Game/BT/AICharacterBase.AICharacterBase_C|SetAdditionalMaxHP _target_3 (+ (Variables|/Game/BT/AICharacterBase.AICharacterBase_C|GetAdditionalMaxHP _target_3) (Math|Float|SelectFloat (* _returnvalue_4 0.5) _returnvalue_4 (Utilities|Array|ContainsItem (Variables|/Game/BT/AICharacterBase.AICharacterBase_C|GetCCs _target_2) "NewEnumerator4")))))
          (Default|HealCharacter _target_2 _returnvalue_4)
          (Variables|/Game/BT/AICharacterBase.AICharacterBase_C|SetBuffedAD _target (+ (Variables|/Game/BT/AICharacterBase.AICharacterBase_C|GetBuffedAD _target) 2e+01))
          (bind _returnvalue_5 (Utilities|Time|SetTimerbyEvent (delegate Custom|Active_Heal) 0.5 true))
          (Variables|Default|SetHealTickEnd _returnvalue_5)
          (EventDispatchers|AssignCharDead (Variables|Default|GetTarget) (delegate Custom|DeactiveHeal)))))))

(event Custom|Active_Heal
  (bind _target (Variables|Default|GetTarget))
  (bind _target_2 (Variables|Default|GetTarget))
  (bind _level (Variables|Default|GetLevel))
  (bind _character (Variables|Default|GetCharacter))
  (bind _losthp (Default|GetLostHP _target))
  (bind _returnvalue (* _level 0.005))
  (bind _healeffectbuff (Variables|/Game/BT/AICharacterBase.AICharacterBase_C|GetHealEffectBuff _character))
  (bind _returnvalue_2 (* _losthp _returnvalue))
  (bind _returnvalue_3 (* _returnvalue_2 _healeffectbuff))
  (if (Variables|/Game/BT/AICharacterBase.AICharacterBase_C|GetIsDead _target)
    (CallFunction|DeactiveHeal :!label _label)
    (else
      (if (== (Variables|Default|GetLevel) 5)
        (Variables|/Game/BT/AICharacterBase.AICharacterBase_C|SetAdditionalMaxHP _target_2 (+ (Variables|/Game/BT/AICharacterBase.AICharacterBase_C|GetAdditionalMaxHP _target_2) (Math|Float|SelectFloat (* _returnvalue_3 0.5) _returnvalue_3 (Utilities|Array|ContainsItem (Variables|/Game/BT/AICharacterBase.AICharacterBase_C|GetCCs _target_2) "NewEnumerator4")))))
      (Default|HealCharacter (Variables|Default|GetTarget) _returnvalue_3)
      (bind _result (Math|Integer|IncrementInt (Variables|Default|GetHealTickCount))
        (:%20%20
          (if (== _result 6)
            (goto _label)))))))

(event Custom|DeactiveHeal
  (params (Character :type AI%20Character%20Base%20Object%20Reference))
  (bind _target (Variables|Default|GetTarget))
  (Utilities|Time|ClearandInvalidateTimerbyHandle (Variables|Default|GetHealTickEnd))
  (if (!= (Variables|Default|GetLevel) 5)
    (Variables|/Game/BT/AICharacterBase.AICharacterBase_C|SetBuffedAD _target (+ (Variables|/Game/BT/AICharacterBase.AICharacterBase_C|GetBuffedAD _target) -2e+01)))
  (Actor|DestroyActor))

(event Custom|SetVisible_Multicast
  (Rendering|SetVisibility (Variables|Default|Getdessert) false false))

(event Custom|SetActorLocation_Multicast
  (params (Location :type Vector))
  (Transformation|SetActorLocation Location false false))

(event EventBeginPlay
  (Components|StaticMesh|SetStaticMesh (Variables|Default|Getdessert) (Utilities|Select :Index (Math|Random|RandomInteger 2) :Option%200 "/Game/Marketplace/Downloads/Cakes/Chesebread/SM_Dessert1.SM_Dessert1" :Option%201 "/Game/Marketplace/Downloads/Cakes/Muffin/SM_Dessert2.SM_Dessert2" :Option%202 "/Game/Marketplace/Downloads/Cakes/TeaCake/SM_Dessert3.SM_Dessert3"))
  (Rendering|SetVisibility (Variables|Default|GetParticleSystem) (== (Variables|Default|GetLevel) 5) false))

(fn ConstructionScript)