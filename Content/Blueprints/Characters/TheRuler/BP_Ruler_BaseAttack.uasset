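; The Ruler's basic attack projectile, with server-side hit detection, damage to its assigned Target, a two-second lifetime and multicast impact effects.
; Dynamic material and Niagara parameters tint the projectile, tail and impact.
; With HiddenPassive on, it homes on the Target and stacks a debuff shown by an attached BP_Ruler_HiddenPassive actor.
; The third such hit resets the stack and adds max-HP-based true damage.
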(event OnComponentBeginOverlap(Collision)
  (params (OverlappedComponent :type Primitive%20Component%20Object%20Reference) (OtherActor :type Actor%20Object%20Reference) (OtherComp :type Primitive%20Component%20Object%20Reference) (OtherBodyIndex :type Integer) (bFromSweep :type Boolean) (SweepResult :type Hit%20Result%20Structure%20%28by%20ref%29))
  (bind _target (Variables|Default|GetTarget))
  (bind _target_2 (Variables|Default|GetTarget))
  (bind (_true _hiddenpassiveactor) (CallFunction|TargetHasHiddenPassiveActor _target))
  ;[0 0 0] 히트 판정
  (if (Networking|IsServer)
    (bind _asaicharacter_base (Utilities|Casting|CastToAICharacterBase OtherActor))
    (if (Math|Boolean|ANDBoolean (!= (Variables|/Game/BT/AICharacterBase.AICharacterBase_C|GetTeam _asaicharacter_base) (Variables|/Game/BT/AICharacterBase.AICharacterBase_C|GetTeam (Variables|Default|GetSelfChar))) (not (Variables|/Game/BT/AICharacterBase.AICharacterBase_C|GetIsDead _asaicharacter_base)) (== OtherComp (Variables|/Game/BT/AICharacterBase.AICharacterBase_C|GetHitbox _asaicharacter_base)))
      (CallFunction|MulticastPlayHitEffect)
      (if (Variables|Default|GetHiddenPassive)
        (Default|DealDamageNormal (Variables|Default|GetTarget) (Variables|Default|GetSelfChar) 1.0 false true "BaseAttack")
        (switch int (Default|GetDebuffStack (Variables|Default|GetTarget) "NewEnumerator4")
          (:0
            (if _true
              _
              (else
                (bind _returnvalue (Game|SpawnActorfromClass "/Game/Blueprints/Characters/TheRuler/BP_Ruler_HiddenPassive.BP_Ruler_HiddenPassive_C" (Math|Transform|MakeTransform (- (Transformation|GetActorLocation (Variables|Default|GetTarget)) "0.000000,0.000000,80.000000") "0, 0, 0" "1.000000,1.000000,1.000000") "Undefined" "MultiplyWithRoot" 0 _target 0))
                (Transformation|AttachActorToActor _returnvalue (Variables|Default|GetTarget) "None" "KeepWorld" "KeepWorld" "KeepWorld" true)))
            (Default|AddDebuffStack (Variables|Default|GetTarget) "NewEnumerator4" 1)
            (Default|PlayEffect _hiddenpassiveactor 1)
            (Actor|DestroyActor))
          (:1
            (for _array_element (Actor|GetAttachedActors (Variables|Default|GetTarget) true false)
              (bind _asbp_ruler_hidden_passive (Utilities|Casting|CastToBP_Ruler_HiddenPassive _array_element))
              (Default|PlayEffect _asbp_ruler_hidden_passive 2))
            (Default|AddDebuffStack (Variables|Default|GetTarget) "NewEnumerator4" 1)
            (Actor|DestroyActor))
          (:2
            (for _array_element_2 (Actor|GetAttachedActors (Variables|Default|GetTarget) true false)
              (bind _asbp_ruler_hidden_passive_2 (Utilities|Casting|CastToBP_Ruler_HiddenPassive _array_element_2))
              (Default|PlayEffect _asbp_ruler_hidden_passive_2 3))
            (Default|ChangeDebuffStack _target_2 "NewEnumerator4")
            (Default|DealDamagebyValue _target_2 (Variables|Default|GetSelfChar) (* (Default|GetMaxHP _target_2) 0.7) true true "BaseAttack")
            (Actor|DestroyActor)))
        (else
          (Default|DealDamageNormal (Variables|Default|GetTarget) (Variables|Default|GetSelfChar) 1.0 false true "BaseAttack")
          (Actor|DestroyActor))))))

(event Custom|Multicast_PlayHitEffect
  (bind _returnvalue (Niagara|SpawnSystematLocation (select (Variables|Default|GetHiddenPassive) "/Game/Marketplace/Hack_And_Slash_FX/VFX_Niagara/Impacts/NS_Ruler_Ult_Hit.NS_Ruler_Ult_Hit" "/Game/FX/BaseRangedAttack/NS_BaseProjectile_Imapact.NS_BaseProjectile_Imapact") (Transformation|GetActorLocation) (Transformation|GetActorRotation)))
  ;[0 0 0] 히트 될 때, 스폰되는 이펙트 색 조정
  (Effects|Components|ParticleSystem|SetColorParameter _returnvalue "Impact_Color" (Variables|Default|GetImpactColor)))

(event EventBeginPlay
  (Utilities|FlowControl|Sequence
    (:then_0
      (bind _returnvalue (Rendering|Material|CreateDynamicMaterialInstance "/Game/FX/BaseRangedAttack/MI_BaseProjectile.MI_BaseProjectile" "None" "None" :!class /Script/Engine.KismetMaterialLibrary))
      (Variables|Default|SetMI_Projectile%20Material _returnvalue)
      (Rendering|Material|SetMaterial (Variables|Default|GetStaticMesh_Projectile) 0 _returnvalue)
      ;[0 0 0] 컬러 조정
      ;;[0 0 0] 투사체 컬러
      (Rendering|Material|SetVectorParameterValue (Variables|Default|GetMI_Projectile%20Material) "Color" (Variables|Default|GetProjectileColor) :!class /Script/Engine.MaterialInstanceDynamic)
      ;;[0 0 0] 꼬리 컬러
      (Effects|Components|ParticleSystem|SetColorParameter (Variables|Default|GetNiagara_Tail) "TailColor" (Variables|Default|GetTailColor)))
    (:then_1
      (Utilities|FlowControl|Delay 2.0)
      (if (Networking|IsServer)
        (Actor|DestroyActor)))))

(event EventTick
  (params (DeltaSeconds :type Float%20%28single-precision%29))
  (bind _projectilemovement (Variables|Default|GetProjectileMovement))
  (if (Networking|IsServer)
    (if (Variables|Default|GetHiddenPassive)
      (if (Variables|/Game/BT/AICharacterBase.AICharacterBase_C|GetIsDead (Variables|Default|GetTarget))
        (Variables|/Script/Engine.MovementComponent|SetVelocity (Variables|Default|GetProjectileMovement) (* (Math|Vector|Normalize (Variables|/Script/Engine.MovementComponent|GetVelocity _projectilemovement)) 6e+03))
        (else
          (Variables|/Script/Engine.MovementComponent|SetVelocity _projectilemovement (* (Math|Vector|Normalize (- (Transformation|GetActorLocation (Variables|Default|GetTarget)) (Transformation|GetActorLocation))) 6e+03)))))))

(fn ConstructionScript)

(fn TargetHasHiddenPassiveActor
  (params (Target :type AI%20Character%20Base%20Object%20Reference))
  (for _array_element (Actor|GetAttachedActors Target true false)
    (bind _asbp_ruler_hidden_passive (Utilities|Casting|CastToBP_Ruler_HiddenPassive _array_element))
    (LocalVariables|SetHasActor true)
    (LocalVariables|SetNewLocalVar _asbp_ruler_hidden_passive))
  (return (LocalVariables|GetHasActor) (LocalVariables|GetNewLocalVar)))