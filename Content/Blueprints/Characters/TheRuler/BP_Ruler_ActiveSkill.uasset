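; The Ruler's active skill projectile, which homes in on a target character and deals damage that grows with its time in flight.
; The server steers it every tick, destroys it if the target is lost, and resolves hits only on that target's Hitbox.
; From caster level 5, hits build debuff stacks shown by an attached BP_Ruler_HiddenPassive.
; The third hit resets the stack and deals true damage based on max HP.
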(event OnComponentBeginOverlap(Sphere)
  (params (OverlappedComponent :type Primitive%20Component%20Object%20Reference) (OtherActor :type Actor%20Object%20Reference) (OtherComp :type Primitive%20Component%20Object%20Reference) (OtherBodyIndex :type Integer) (bFromSweep :type Boolean) (SweepResult :type Hit%20Result%20Structure%20%28by%20ref%29))
  (bind _target (Variables|Default|GetTarget))
  (bind _target_2 (Variables|Default|GetTarget))
  (bind _target_3 (Variables|Default|GetTarget))
  (if (Networking|IsServer)
    (if (and (== OtherActor _target_3) (== OtherComp (Variables|/Game/BT/AICharacterBase.AICharacterBase_C|GetHitbox _target_3)))
      (Default|DealDamageNormal (Variables|Default|GetTarget) (Variables|Default|GetSelfChar) (+ (* (Actor|GetGameTimeSinceCreation) 12.0) 1.0) false true "None")
      (CallFunction|PlayEffect)
      (if (>= (Variables|/Game/BT/AICharacterBase.AICharacterBase_C|GetLevel (Variables|Default|GetSelfChar)) 5)
        (switch int (Default|GetDebuffStack (Variables|Default|GetTarget) "NewEnumerator4")
          (:0
            (bind _returnvalue (Game|SpawnActorfromClass "/Game/Blueprints/Characters/TheRuler/BP_Ruler_HiddenPassive.BP_Ruler_HiddenPassive_C" (Math|Transform|MakeTransform (- (Transformation|GetActorLocation _target) "0.000000,0.000000,80.000000") "0, 0, 0" "1.000000,1.000000,1.000000") "Undefined" "MultiplyWithRoot" 0 _target 0))
            (Transformation|AttachActorToActor _returnvalue (Variables|Default|GetTarget) "None" "KeepWorld" "KeepWorld" "KeepWorld" true)
            (Default|AddDebuffStack (Variables|Default|GetTarget) "NewEnumerator4" 1)
            (Default|PlayEffect _returnvalue 1)
            (Actor|DestroyActor))
          (:1
            (for _array_element (Actor|GetAttachedActors (Variables|Default|GetTarget) true false)
              (bind _asbp_ruler_hidden_passive (Utilities|Casting|CastToBP_Ruler_HiddenPassive _array_element))
              (Default|PlayEffect _asbp_ruler_hidden_passive 2))
            (Default|AddDebuffStack (Variables|Default|GetTarget) "NewEnumerator4" 1)
            (Actor|DestroyActor))
          (:2
            (for _array_element_2 (Actor|GetAttachedActors (Variables|Default|GetTarget) true false)
              (bind _asbp_ruler_hidden_passive_2 (Utilities|Casting|CastToBP_Ruler_HiddenPassive _array_element_2))
              (Default|PlayEffect _asbp_ruler_hidden_passive_2 3))
            (Default|ChangeDebuffStack _target_2 "NewEnumerator4")
            (Default|DealDamagebyValue _target_2 (Variables|Default|GetSelfChar) (* (Default|GetMaxHP _target_2) 0.7) true true "BaseAttack")
            (Actor|DestroyActor)))
        (else
          (Actor|DestroyActor))))))

(event Custom|커스텀이벤트)

(event Custom|PlayEffect
  (Niagara|SpawnSystematLocation "/Game/FX/H_M_SHIN/GolfSwing/NS_Golf_Impact.NS_Golf_Impact" (Transformation|GetActorLocation)))

(event EventBeginPlay
  (Niagara|SpawnSystematLocation "/Game/FX/H_M_SHIN/GolfSwing/NS_Golf_Impact.NS_Golf_Impact" (Transformation|GetActorLocation) (Math|Conversions|RotationFromXVector (Transformation|GetActorForwardVector))))

(event Collision|EventActorBeginOverlap
  (params (OtherActor :type Actor%20Object%20Reference)))

(event EventTick
  (params (DeltaSeconds :type Float%20%28single-precision%29))
  (bind _returnvalue (Transformation|GetActorLocation))
  (bind _target (Variables|Default|GetTarget))
  (bind _returnvalue_2 (Transformation|GetActorLocation _target))
  (if (Networking|IsServer)
    (Utilities|IsValid _target
      (:Is%20Valid
        (Variables|/Script/Engine.MovementComponent|SetVelocity (Variables|Default|GetProjectileMovement) (* (Math|Vector|Normalize (- _returnvalue_2 _returnvalue)) 6e+03))
        (Transformation|SetActorRotation (Math|Rotator|FindLookatRotation _returnvalue _returnvalue_2)))
      (:Is%20Not%20Valid
        (Actor|DestroyActor)))))

(fn ConstructionScript)