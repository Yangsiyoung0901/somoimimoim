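; The Ruler, an AI combat character whose skills spawn separate actors for basic attack, active skill and ultimate.
; Active skill targets the farthest enemy; basic attack gains a hidden passive and color change at level 5.
; From level 3, any other character's death stacks move and attack speed buffs.
; A server-side tick arms the ultimate once three allies, itself included, are nearby; it buffs them while the Ruler is immune and unstoppable.
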(event Custom|ActiveSkill
  (bind _returnvalue (Transformation|GetActorLocation))
  (bind _farthesttarget (CallFunction|GetFarthestEnemy))
  (Utilities|IsValid _farthesttarget
    (:Is%20Valid
      (Game|SpawnActorfromClass "/Game/Blueprints/Characters/TheRuler/BP_Ruler_ActiveSkill.BP_Ruler_ActiveSkill_C" (Math|Transform|MakeTransform _returnvalue (Math|Rotator|FindLookatRotation _returnvalue (Transformation|GetActorLocation _farthesttarget)) "1.000000,1.000000,1.000000") "Undefined" "MultiplyWithRoot" 0 _farthesttarget self 0))))

(event Custom|UltSkill
  (Variables|Default|SetUltSkillCondition false)
  (Variables|Default|SetIsImmune true)
  (Variables|Default|SetIsUnstoppable true)
  (bind _nearalies (CallFunction|GetAlliesinRange 1.25e+03))
  (Game|SpawnActorfromClass "/Game/Blueprints/Characters/TheRuler/BP_Ruler_Ult.BP_Ruler_Ult_C" (Math|Transform|MakeTransform (- (Transformation|GetActorLocation) "0.000000,0.000000,88.000000") "0, 0, 0" "1.000000,1.000000,1.000000") "Undefined" "MultiplyWithRoot" 0 _nearalies 0)
  (EventDispatchers|AssignOnUltEnd (delegate Custom|OnUltEnd_이벤트)))

(event Custom|BaseAttack
  (bind _returnvalue (Transformation|GetActorLocation))
  (bind _level (Variables|Default|GetLevel))
  (bind _returnvalue_2 (>= _level 5))
  (bind _returnvalue_3 (Math|Color|SelectColor "(R=20.000000,G=0.173619,B=0.000000,A=1.000000)" "(R=10.000000,G=10.000000,B=10.000000,A=1.000000)" _returnvalue_2))
  (bind _attacktarget (Variables|Default|GetAttackTarget)
    (:then
      (Game|SpawnActorfromClass "/Game/Blueprints/Characters/TheRuler/BP_Ruler_BaseAttack.BP_Ruler_BaseAttack_C" (Math|Transform|MakeTransform _returnvalue (Math|Rotator|FindLookatRotation _returnvalue (Transformation|GetActorLocation _attacktarget)) "1.000000,1.000000,1.000000") "Undefined" "MultiplyWithRoot" 0 false _returnvalue_3 _returnvalue_3 _returnvalue_3 self _attacktarget _returnvalue_2 0))
    (:else)))

(event Custom|PassiveSkill
  (if (not (Variables|Default|GetIsDead))
    (Variables|Default|SetBuffSpeed (+ (Variables|Default|GetBuffSpeed) 3e+01))
    (Variables|Default|SetBuffAS (+ (Variables|Default|GetBuffAS) 3e+01))
    (CallFunction|ApplyStatChange)
    (CallFunction|PlayEffect)))

(event Custom|CharDead_이벤트
  ;[1 1 1] 전투 시작 시, 적과 아군에게 바인딩하는걸로 수정 필요
  (if (>= (Variables|Default|GetLevel) 3)
    (CallFunction|PassiveSkill)))

(event Custom|OnUltEnd_이벤트
  (Variables|Default|SetIsImmune false)
  (Variables|Default|SetIsUnstoppable false))

(event Custom|PlayEffect
  (Niagara|SpawnSystemAttached "/Game/FX/H_M_SHIN/MyManIsPrecious/NS_MyManIsPrecious.NS_MyManIsPrecious" (Variables|Character|GetMesh) "None" (- (Transformation|GetActorLocation) "0.000000,0.000000,80.000000") "0, 0, 0" "KeepWorldPosition" false))

(event Collision|EventActorBeginOverlap
  (params (OtherActor :type Actor%20Object%20Reference))
  (|CallParentFunction OtherActor) ; 지금 이 노드는 비활성 상태입니다. \n핀을 끌어서 다른 노드를 연결하면 활성화됩니다.
)

(event EventTick
  (params (DeltaSeconds :type Float%20%28single-precision%29))
  (|CallParentFunction DeltaSeconds)
  (if (Networking|IsServer)
    (bind _nearalies (CallFunction|GetAlliesinRange 1.25e+03))
    (if (>= (Utilities|Array|Length _nearalies) 3)
      (Utilities|FlowControl|DoOnce false
        (:Completed
          (Variables|Default|SetUltSkillCondition true))))))

(event EventBeginPlay
  ;[1 1 1] 전투 시작 시, 적과 아군에게 바인딩하는걸로 수정 필요
  (|CallParentFunction)
  (bind _outactors (Actor|GetAllActorsOfClass "/Game/BT/AICharacterBase.AICharacterBase_C"))
  (for _array_element _outactors
    (if (!= _array_element self)
      (EventDispatchers|AssignCharDead _array_element (delegate Custom|CharDead_이벤트)))))

(fn ConstructionScript
  (|CallParentFunction))

(fn GetFarthestEnemy
  (bind _returnvalue (Transformation|GetActorLocation))
  (LocalVariables|SetFarthestLocation (Transformation|GetActorLocation))
  (for _array_element (CallFunction|GetAllAliveEnemy)
    (if (>= (Math|Vector|Distance(Vector) _returnvalue (Transformation|GetActorLocation _array_element)) (Math|Vector|Distance(Vector) _returnvalue (LocalVariables|GetFarthestLocation)))
      (LocalVariables|SetFarthestLocation (Transformation|GetActorLocation _array_element))
      (LocalVariables|SetTempTarget _array_element)))
  (return (LocalVariables|GetTempTarget)))

(fn GetAlliesinRange
  (params (Range :type Float%20%28double-precision%29))
  (for _array_element (CallFunction|GetAllAliveAllies)
    (if (<= (CallFunction|GetDistancewithTarget _array_element) Range)
      (Utilities|Array|Add (LocalVariables|GetNearCharacter) _array_element)))
  (Utilities|Array|Add (LocalVariables|GetNearCharacter) self)
  (return (LocalVariables|GetNearCharacter)))