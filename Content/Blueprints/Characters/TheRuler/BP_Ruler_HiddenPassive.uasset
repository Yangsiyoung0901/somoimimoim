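; BP_Ruler_HiddenPassive is the "YouOut" stack indicator for the Ruler's hidden passive, built from two rings and an impact effect.
; PlayEffect dispatches on stack: one grows the inner ring and tints both yellow, two grows the outer ring and tints both red, three collapses both and fires the Niagara impact.
; Looping timers animate scale, dynamic materials carry color, and the server destroys the actor when its Target is destroyed.
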(event Custom|Hit1
  (bind _returnvalue (Utilities|Time|SetTimerbyEvent (delegate Custom|Event_Hit1) 0.01 true))
  (Variables|Default|SetTimer_Hit1 _returnvalue)
  (Components|Activation|SetActive (Variables|Default|GetNS_YouOut_Impact) false false)
  (Utilities|FlowControl|DelayUntilNextTick)
  (Rendering|Material|SetVectorParameterValue (Variables|Default|GetInnerColor) "color" "(R=1.000000,G=1.000000,B=0.000000,A=1.000000)" :!class /Script/Engine.MaterialInstanceDynamic))

(event Custom|Hit2
  (bind _returnvalue (Utilities|Time|SetTimerbyEvent (delegate Custom|Event_Hit2) 0.01 true))
  (Variables|Default|SetTimer_Hit2 _returnvalue)
  (Rendering|Material|SetVectorParameterValue (Variables|Default|GetInnerColor) "color" "(R=1.000000,G=0.000000,B=0.000000,A=1.000000)" :!class /Script/Engine.MaterialInstanceDynamic))

(event Custom|Event_Hit1
  (Transformation|SetRelativeScale3D (Variables|Default|GetRing1) (Math|Vector|MakeVector (Variables|Default|GetScale_Ring1) (Variables|Default|GetScale_Ring1) 1.0))
  (if (> (Variables|Default|GetScale_Ring1) 0.7)
    (Utilities|Time|ClearandInvalidateTimerbyHandle (Variables|Default|GetTimer_Hit1))
    (else
      (Variables|Default|SetScale_Ring1 (+ (Variables|Default|GetScale_Ring1) 0.07)))))

(event Custom|Event_Hit2
  (Transformation|SetRelativeScale3D (Variables|Default|GetRing2) (Math|Vector|MakeVector (Variables|Default|GetScale_Hit2) (Variables|Default|GetScale_Hit2) 1.0))
  (if (> (Variables|Default|GetScale_Hit2) 1.0)
    (Utilities|Time|ClearandInvalidateTimerbyHandle (Variables|Default|GetTimer_Hit2))
    (else
      (Variables|Default|SetScale_Hit2 (+ (Variables|Default|GetScale_Hit2) 0.1)))))

(event Custom|Hit3
  (Transformation|SetRelativeScale3D (Variables|Default|GetRing1) (Math|Vector|MakeVector 0.0 0.0 1.0))
  (Transformation|SetRelativeScale3D (Variables|Default|GetRing2) (Math|Vector|MakeVector 0.0 0.0 1.0))
  (Variables|Default|SetScale_Ring1 0.0)
  (Variables|Default|SetScale_Hit2 0.0)
  (Components|Activation|SetActive (Variables|Default|GetNS_YouOut_Impact) true false))

(event Custom|PlayEffect
  (params (Stack :type Integer))
  (switch int Stack
    (:1
      (CallFunction|Hit1))
    (:2
      (CallFunction|Hit2))
    (:3
      (CallFunction|Hit3))))

(event Custom|OnDestroyed_이벤트
  (params (DestroyedActor :type Actor%20Object%20Reference))
  (Actor|DestroyActor))

(event Collision|EventActorBeginOverlap
  (params (OtherActor :type Actor%20Object%20Reference)))

(event EventTick
  (params (DeltaSeconds :type Float%20%28single-precision%29)))

(event EventBeginPlay
  (bind _returnvalue (Rendering|Material|CreateDynamicMaterialInstance (Variables|Default|GetRing1) 0 "/Game/FX/H_M_SHIN/YouOut/M_YouOut_Ring.M_YouOut_Ring" "None" :!class /Script/Engine.PrimitiveComponent))
  (Variables|Default|SetInnerColor _returnvalue)
  (bind _returnvalue_2 (Rendering|Material|CreateDynamicMaterialInstance (Variables|Default|GetRing2) 0 "/Game/FX/H_M_SHIN/YouOut/M_YouOut_Ring.M_YouOut_Ring" "None" :!class /Script/Engine.PrimitiveComponent))
  (Variables|Default|SetOuterColor _returnvalue_2)
  (if (Networking|IsServer)
    (Game|AssignOnDestroyed (Variables|Default|GetTarget) (delegate Custom|OnDestroyed_이벤트))))

(fn ConstructionScript)