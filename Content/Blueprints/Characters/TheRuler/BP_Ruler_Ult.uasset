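; BP_Ruler_Ult is the Ruler's ultimate, a temporary buff for every character in its BuffChar array.
; On BeginPlay it adds flat attack damage, attack speed and movement speed bonuses, calling each character's change handlers, then subtracts them after an eight-second delay.
; BuffChar is not filled within this Blueprint.
; The DestroyActor node is unconnected, so the actor does not destroy itself afterward.
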(event EventBeginPlay
  (for _array_element (Variables|Default|GetBuffChar)
    (Variables|/Game/BT/AICharacterBase.AICharacterBase_C|SetBuffedAD _array_element (+ (Variables|/Game/BT/AICharacterBase.AICharacterBase_C|GetBuffedAD _array_element) 5e+01))
    (Variables|/Game/BT/AICharacterBase.AICharacterBase_C|SetBuffAS _array_element (+ (Variables|/Game/BT/AICharacterBase.AICharacterBase_C|GetBuffAS _array_element) 5e+01))
    (Default|AttackSpeedChanged _array_element)
    (Variables|/Game/BT/AICharacterBase.AICharacterBase_C|SetBuffSpeed _array_element (+ (Variables|/Game/BT/AICharacterBase.AICharacterBase_C|GetBuffSpeed _array_element) 5e+01))
    (Default|SpeedChanged _array_element))
  (Utilities|FlowControl|Delay 8.0)
  (for _array_element_2 (Variables|Default|GetBuffChar)
    (Variables|/Game/BT/AICharacterBase.AICharacterBase_C|SetBuffedAD _array_element_2 (+ (Variables|/Game/BT/AICharacterBase.AICharacterBase_C|GetBuffedAD _array_element_2) -5e+01))
    (Variables|/Game/BT/AICharacterBase.AICharacterBase_C|SetBuffAS _array_element_2 (+ (Variables|/Game/BT/AICharacterBase.AICharacterBase_C|GetBuffAS _array_element_2) -5e+01))
    (Default|AttackSpeedChanged _array_element_2)
    (Variables|/Game/BT/AICharacterBase.AICharacterBase_C|SetBuffSpeed _array_element_2 (+ (Variables|/Game/BT/AICharacterBase.AICharacterBase_C|GetBuffSpeed _array_element_2) -5e+01))
    (Default|SpeedChanged _array_element_2)))

(event Collision|EventActorBeginOverlap
  (params (OtherActor :type Actor%20Object%20Reference)))

(event EventTick
  (params (DeltaSeconds :type Float%20%28single-precision%29)))

(fn ConstructionScript)