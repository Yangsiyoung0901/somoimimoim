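; Villain battle character, an assassin with level-gated abilities that hunts the lowest-HP enemy.
; The active skill vanishes and teleports beside that enemy, with a separate event dealing true damage.
; Hits apply CC at level 3 and, from level 4, arm the ult on badly wounded targets, granting immunity until it fires.
; The ult executes low-HP enemies in a frontal area and damages others; level 5 adds avoidance through a hidden passive.
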(event Custom|Active_Attack
  (bind _target (CallFunction|GetLowestHpEnemy))
  (Utilities|IsValid _target
    (:Is%20Valid
      (CallFunction|ActiveSkillEffect false (Transformation|GetActorLocation _target))
      (Default|DealDamageNormal _target self 2.5 true true "None")
      (Utilities|FlowControl|Sequence
        (:then_0
          (bind _ulttarget (CallFunction|CheckUltCondition _target))
          (Utilities|IsValid _ulttarget
            (:Is%20Valid
              (Variables|Default|SetUltTarget _ulttarget)
              (Variables|Default|SetUltSkillCondition true)
              (Variables|Default|SetIsUnstoppable true)
              (Variables|Default|SetIsImmune true)
              (Default|RemoveAllCCs (Variables|Default|GetBPC_CCs)))))
        (:then_1
          (if (>= (Variables|Default|GetLevel) 3)
            (Variables|Default|SetRecentAttackTarget _target)
            (Default|ApplyCC (Variables|/Game/BT/AICharacterBase.AICharacterBase_C|GetBPC_CCs _target) "NewEnumerator0" 1.5)))))))

(event Custom|ActiveSkillEffect
  (params (Teleport :type Boolean) (Location :type Vector))
  (if Teleport
    (Effects|SpawnEmitteratLocation "/Game/ImpactFX/ParticleSystems/Par_CloudImpact_Collection_01.Par_CloudImpact_Collection_01" (- (Transformation|GetActorLocation) "0.000000,0.000000,60.000000"))
    (else
      (Effects|SpawnEmitteratLocation "/Game/ImpactFX/ParticleSystems/Par_Various_Collection_1.Par_Various_Collection_1" Location))))

(event Custom|HiddenPassiveEffect
  (params (ON :type Boolean))
  (bind _hiddenpassive (Variables|Default|GetHiddenPassive))
  (if ON
    (Components|Activation|Activate _hiddenpassive true)
    (else
      (Components|Activation|Deactivate _hiddenpassive))))

(event EventBeginPlay
  (|CallParentFunction) ; 지금 이 노드는 비활성 상태입니다. \n핀을 끌어서 다른 노드를 연결하면 활성화됩니다.
)

(event Collision|EventActorBeginOverlap
  (params (OtherActor :type Actor%20Object%20Reference))
  (|CallParentFunction OtherActor) ; 지금 이 노드는 비활성 상태입니다. \n핀을 끌어서 다른 노드를 연결하면 활성화됩니다.
)

(event EventTick
  (params (DeltaSeconds :type Float%20%28single-precision%29))
  (|CallParentFunction DeltaSeconds) ; 지금 이 노드는 비활성 상태입니다. \n핀을 끌어서 다른 노드를 연결하면 활성화됩니다.
)

(event EventBaseAttack
  (bind _attacktarget (Variables|Default|GetAttackTarget))
  (bind _attacktarget_2 (Variables|Default|GetAttackTarget))
  (bind _attacktarget_3 (Variables|Default|GetAttackTarget))
  (Variables|Default|GetAttackTarget
    (:then
      (Default|DealDamageNormal _attacktarget self 1.0 false true "BaseAttack")
      (Utilities|FlowControl|Sequence
        (:then_0
          (bind _ulttarget (CallFunction|CheckUltCondition _attacktarget))
          (Utilities|IsValid _ulttarget
            (:Is%20Valid
              (Variables|Default|SetUltTarget _ulttarget)
              (Variables|Default|SetUltSkillCondition true)
              (Variables|Default|SetIsUnstoppable true)
              (Variables|Default|SetIsImmune true)
              (Default|RemoveAllCCs (Variables|Default|GetBPC_CCs)))))
        (:then_1
          (if (>= (Variables|Default|GetLevel) 3)
            (bind _recentattacktarget (Variables|Default|GetRecentAttackTarget)
              (:then
                (if (not (== _recentattacktarget (Variables|Default|GetAttackTarget)))
                  (Variables|Default|SetRecentAttackTarget _attacktarget_2)
                  (Default|ApplyCC (Variables|/Game/BT/AICharacterBase.AICharacterBase_C|GetBPC_CCs _attacktarget_2) "NewEnumerator0" 2.0)))
              (:else
                (Variables|Default|SetRecentAttackTarget _attacktarget_3)
                (Default|ApplyCC (Variables|/Game/BT/AICharacterBase.AICharacterBase_C|GetBPC_CCs _attacktarget_3) "NewEnumerator0" 1.5)))))))
    (:else)))

(event EventActiveSkill
  (bind _returnvalue (Transformation|GetActorLocation))
  (Variables|Default|SetIsUnstoppable true)
  (Variables|Default|SetIsImmune true)
  (CallFunction|ActiveSkillEffect true "0, 0, 0")
  (CallFunction|SetCharUnblocked true)
  (if (Variables|Default|GetbHidden)
    _
    (else
      (Rendering|SetActorHiddenInGame true)))
  (Utilities|FlowControl|Delay 0.15)
  (bind _target (CallFunction|GetLowestHpEnemy))
  (Utilities|IsValid _target
    (:Is%20Valid
      (Transformation|SetActorLocation (Math|Vector|MakeVector (.X (Math|Vector|BreakVector (.ProjectedLocation (AI|Navigation|ProjectPointtoNavigation (+ (* (Math|Vector|Normalize (Math|Vector|ProjectVectorontoPlane (Math|Random|RandomUnitVector) "0.000000,0.000000,1.000000")) 2.5e+02) (Transformation|GetActorLocation _target)) 0 0 "250.000000,250.000000,250.000000")))) (.Y (Math|Vector|BreakVector (.ProjectedLocation (AI|Navigation|ProjectPointtoNavigation (+ (* (Math|Vector|Normalize (Math|Vector|ProjectVectorontoPlane (Math|Random|RandomUnitVector) "0.000000,0.000000,1.000000")) 2.5e+02) (Transformation|GetActorLocation _target)) 0 0 "250.000000,250.000000,250.000000")))) (.Z (Math|Vector|BreakVector _returnvalue))) false false)
      (Transformation|SetActorRotation (Math|Rotator|FindLookatRotation _returnvalue (Transformation|GetActorLocation _target))))
    (:Is%20Not%20Valid
      _))
  (if (Variables|Default|GetbHidden)
    (Rendering|SetActorHiddenInGame false))
  (CallFunction|ActiveSkillEffect true "0, 0, 0")
  (Variables|Default|SetIsUnstoppable false)
  (Variables|Default|SetIsImmune false)
  (CallFunction|SetCharUnblocked false))

(event EventUltSkill
  (bind _self self)
  (Variables|Default|SetUltSkillCondition false)
  (Variables|Default|SetIsUnstoppable false)
  (Variables|Default|SetIsImmune false)
  (bind _nearenemies (CallFunction|UltGetEnemy (+ (* (Transformation|GetActorForwardVector) 2.5e+02) (Transformation|GetActorLocation)) 3e+02))
  (for _array_element _nearenemies
    (if (>= (.Percentage (Default|GetLostHP _array_element)) 7e+01)
      (Default|DealDamagebyValue _array_element _self (Default|GetMaxHP _array_element) true false "None")
      (else
        (Default|DealDamagebyValue _array_element _self (* (Default|GetMaxHP _array_element) 0.3) false false "None")))))

(event EventBattleStartServer
  (|CallParentFunction)
  (if (>= (Variables|Default|GetLevel) 5)
    (Variables|Default|SetAvoidRate (+ (Variables|Default|GetAvoidRate) 1e+02))
    (Variables|Default|SetHiddenPassiveOn true)
    (CallFunction|HiddenPassiveEffect true)
    (elif (Variables|Default|GetHiddenPassiveOn)
      (Variables|Default|SetAvoidRate (+ (Variables|Default|GetAvoidRate) -1e+02))
      (Variables|Default|SetHiddenPassiveOn false)
      (CallFunction|HiddenPassiveEffect false))))

(event EventLevelChange
  (params (Level :type Integer))
  (|CallParentFunction Level)
  (if (>= (Variables|Default|GetLevel) 5)
    (Variables|Default|SetAvoidRate (+ (Variables|Default|GetAvoidRate) 1e+02))
    (Variables|Default|SetHiddenPassiveOn true)
    (CallFunction|HiddenPassiveEffect true)
    (elif (Variables|Default|GetHiddenPassiveOn)
      (Variables|Default|SetAvoidRate (+ (Variables|Default|GetAvoidRate) -1e+02))
      (Variables|Default|SetHiddenPassiveOn false)
      (CallFunction|HiddenPassiveEffect false))))

(fn ConstructionScript
  (|CallParentFunction))

(fn GetLowestHpEnemy
  (for _array_element (CallFunction|GetAllAliveEnemy)
    (if (<= (Variables|/Game/BT/AICharacterBase.AICharacterBase_C|GetCurrentHP _array_element) (LocalVariables|GetLowestHP))
      (LocalVariables|SetLowestHP (Variables|/Game/BT/AICharacterBase.AICharacterBase_C|GetCurrentHP _array_element))
      (LocalVariables|SetActiveSkillTarget _array_element)))
  (return (LocalVariables|GetActiveSkillTarget)))

(fn CheckUltCondition
  (params (CheckEnemy :type AI%20Character%20Base%20Object%20Reference))
  (bind _percentage (Default|GetLostHP CheckEnemy))
  (if (>= (Variables|Default|GetLevel) 4)
    (if (and (>= _percentage 7e+01) (<= _percentage 99.0))
      (return CheckEnemy)
      (else
        _)))
  (return 0))

(fn UltGetEnemy
  (params (Location :type Vector) (Range :type Float%20%28double-precision%29))
  (for _array_element (CallFunction|GetAllAliveEnemy)
    (if (<= (Math|Vector|Distance(Vector) (Transformation|GetActorLocation _array_element) Location) Range)
      (Utilities|Array|Add (LocalVariables|GetEnemyInDistance) _array_element)))
  (return (LocalVariables|GetEnemyInDistance)))