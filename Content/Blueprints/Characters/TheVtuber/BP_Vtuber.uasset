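; Vtuber tank character with level-gated skills, built on a parent with shared combat events.
; Passives reflect damage with CC on attackers and raise armor as health drops; the active ticks missing-health healing below half HP.
; Lethal damage can trigger a last-stand ultimate: immune, heal-banned, CCing nearby enemies, then dying when it ends.
; A hidden aura makes overlapping allies ignore damage, redirecting part to itself as true damage via event bindings.
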(event OnComponentBeginOverlap(HiddenPassiveCollision)
  (params (OverlappedComponent :type Primitive%20Component%20Object%20Reference) (OtherActor :type Actor%20Object%20Reference) (OtherComp :type Primitive%20Component%20Object%20Reference) (OtherBodyIndex :type Integer) (bFromSweep :type Boolean) (SweepResult :type Hit%20Result%20Structure%20%28by%20ref%29))
  (bind _asaicharacter_base (Utilities|Casting|CastToAICharacterBase OtherActor))
  (if (Utilities|Array|ContainsItem (CallFunction|GetAllAliveAllies) _asaicharacter_base)
    (Variables|/Game/BT/AICharacterBase.AICharacterBase_C|SetIgnoreDamage _asaicharacter_base true)
    (EventDispatchers|AssignApplyDamageTriggered _asaicharacter_base (delegate Custom|ApplyDamageTriggered_이벤트))))

(event OnComponentEndOverlap(HiddenPassiveCollision)
  (params (OverlappedComponent :type Primitive%20Component%20Object%20Reference) (OtherActor :type Actor%20Object%20Reference) (OtherComp :type Primitive%20Component%20Object%20Reference) (OtherBodyIndex :type Integer))
  (bind _asaicharacter_base (Utilities|Casting|CastToAICharacterBase OtherActor))
  (if (Utilities|Array|ContainsItem (CallFunction|GetAllAliveAllies) _asaicharacter_base)
    (Variables|/Game/BT/AICharacterBase.AICharacterBase_C|SetIgnoreDamage _asaicharacter_base false)
    (EventDispatchers|UnbindEventfromApplyDamageTriggered _asaicharacter_base (delegate Custom|ApplyDamageTriggered_이벤트))))

(event Custom|OnActiveSkillEnd_이벤트
  ;[1 1 1] 액티브 - 도트힐
  (Components|Activation|Deactivate (Variables|Default|GetActiveHeal))
  (Utilities|Time|ClearandInvalidateTimerbyHandle (Variables|Default|GetActiveSkillTimer)))

(event Custom|Active_Heal
  ;[1 1 1] 액티브 - 도트힐
  (if (not (Variables|Default|GetHealBanned))
    (CallFunction|HealCharacter (* (.LostHP (CallFunction|GetLostHP)) 0.15))))

(event Custom|Passive_Reflect
  (params (DamageDealer :type AI%20Character%20Base%20Object%20Reference) (Damage :type Float%20%28double-precision%29) (IsTrueDamage :type Boolean) (Target :type Boolean) (Tag :type Name))
  ;[1 1 1] 패시브
  ;;[1 1 1] 패시브 - 반사, 치감 적용
  (if (>= (Variables|Default|GetLevel) 3)
    (if (!= Tag "Reflect")
      (Default|DealDamagebyValue DamageDealer self (* Damage 0.1) false false "Reflect")
      (Default|ApplyCC (Variables|/Game/BT/AICharacterBase.AICharacterBase_C|GetBPC_CCs DamageDealer) "NewEnumerator4" 3.0))))

(event Custom|End
  ;[1 1 1] 패시브
  (bind _asfx_spark_passive (Utilities|Casting|CastToFX_SPark_Passive (Variables|/Script/Engine.ChildActorComponent|GetChildActor (Variables|Default|GetPassive))))
  (Default|End _asfx_spark_passive))

(event Custom|CharDead_이벤트
  (bind _asfx_im_fine (Utilities|Casting|CastToFX_ImFine (Variables|/Script/Engine.ChildActorComponent|GetChildActor (Variables|Default|GetHiddenPassive))))
  (Default|End _asfx_im_fine)
  (Collision|SetCollisionEnabled (Variables|Default|GetHiddenPassiveCollision) "NoCollision"))

(event Custom|OnUltEnd_이벤트
  (Default|CallCharDead)
  (Variables|Default|SetIsDead true))

(event Custom|ApplyDamageTriggered_이벤트
  (params (Damage :type Float%20%28double-precision%29) (Tag :type Name) (DamageDealer :type AI%20Character%20Base%20Object%20Reference))
  (Default|DealDamagebyValue self DamageDealer (* Damage 0.3) true false "None"))

(event EventBeginPlay
  (bind _hiddenpassive (Variables|Default|GetHiddenPassive))
  (|CallParentFunction)
  (Utilities|FlowControl|Sequence
    (:then_0
      (if (>= (Variables|Default|GetLevel) 5)
        (Rendering|SetVisibility _hiddenpassive true false)
        (bind _asfx_im_fine (Utilities|Casting|CastToFX_ImFine (Variables|/Script/Engine.ChildActorComponent|GetChildActor _hiddenpassive)))
        (Default|Start _asfx_im_fine)
        (EventDispatchers|AssignCharDead (delegate Custom|CharDead_이벤트))
        (Collision|SetCollisionEnabled (Variables|Default|GetHiddenPassiveCollision) "QueryOnly")))
    (:then_1
      ;[1 1 1] 패시브
      (if (>= (Variables|Default|GetLevel) 3)
        (EventDispatchers|BindEventtoUnderAttackTriggered (delegate Custom|Passive_Reflect))
        (bind _asfx_spark_passive (Utilities|Casting|CastToFX_SPark_Passive (Variables|/Script/Engine.ChildActorComponent|GetChildActor (Variables|Default|GetPassive))))
        (Default|Start _asfx_spark_passive)
        (EventDispatchers|BindEventtoCharDead (delegate Custom|End))))))

(event Collision|EventActorBeginOverlap
  (params (OtherActor :type Actor%20Object%20Reference))
  (|CallParentFunction OtherActor) ; 지금 이 노드는 비활성 상태입니다. \n핀을 끌어서 다른 노드를 연결하면 활성화됩니다.
)

(event EventTick
  (params (DeltaSeconds :type Float%20%28single-precision%29))
  (bind _percentage (CallFunction|GetLostHP))
  (bind _returnvalue (Math|Float|Floor _percentage))
  (|CallParentFunction DeltaSeconds)
  (Utilities|FlowControl|Sequence
    (:then_0
      (if (<= (/ (Variables|Default|GetCurrentHP) (CallFunction|GetMaxHP)) 0.5)
        (Variables|Default|SetActiveSkillCondition true)
        (else
          (Variables|Default|SetActiveSkillCondition false))))
    (:then_1
      ;[1 1 1] 패시브 - 잃은 체력 비례 방어력 상승
      (if (>= (Variables|Default|GetLevel) 3)
        (if (!= (Variables|Default|GetCurrentBuffedArmor) _returnvalue)
          (Variables|Default|SetBuffedArmor (+ (Variables|Default|GetBuffedArmor) (Math|Conversions|ToFloat(Integer) (- _returnvalue (Variables|Default|GetCurrentBuffedArmor)))))
          (Variables|Default|SetCurrentBuffedArmor _returnvalue))))))

(event EventBaseAttack
  (bind _attacktarget (Variables|Default|GetAttackTarget)
    (:then
      (Default|DealDamageNormal _attacktarget self 1.0 false true "BaseAttack"))
    (:else)))

(event EventUltSkill
  (bind _self self)
  (Variables|Default|SetIsImmune true)
  (Variables|Default|SetIsUnstoppable true)
  (Variables|Default|SetHealBanned true)
  (Variables|Default|SetUltSkillCondition false)
  (bind _asfx_its_play_time (Utilities|Casting|CastToFX_ItsPlayTime (Variables|/Script/Engine.ChildActorComponent|GetChildActor (Variables|Default|GetUlt))))
  (Default|Start _asfx_its_play_time)
  (for _array_element (CallFunction|GetAllAliveEnemy)
    (if (<= (Transformation|GetDistanceTo _array_element _self) 1e+03)
      (Default|ApplyCC (Variables|/Game/BT/AICharacterBase.AICharacterBase_C|GetBPC_CCs _array_element) "NewEnumerator2" 3.0 _self)))
  (EventDispatchers|AssignOnUltEnd (delegate Custom|OnUltEnd_이벤트)))

(event EventActiveSkill
  ;[1 1 1] 액티브 - 도트힐
  (if (>= (Variables|Default|GetLevel) 2)
    (Components|Activation|Activate (Variables|Default|GetActiveHeal) true)
    (EventDispatchers|AssignOnActiveSkillEnd (delegate Custom|OnActiveSkillEnd_이벤트))
    (bind _returnvalue (Utilities|Time|SetTimerbyEvent (delegate Custom|Active_Heal) 0.5 true))
    (Variables|Default|SetActiveSkillTimer _returnvalue)))

(event EventApplyDamage
  (params (Damage :type Float%20%28double-precision%29) (Tag :type Name :default "None") (DamageDealer :type AI%20Character%20Base%20Object%20Reference))
  (Default|CallApplyDamageTriggered Damage Tag DamageDealer)
  (if (not (Variables|Default|GetIgnoreDamage))
    (bind _output_get (Variables|Default|SetCurrentHP (- (Variables|Default|GetCurrentHP) Damage)))
    (if (<= _output_get 0.0)
      (Default|CallCallDangerOfDeath)
      (if (<= (Variables|Default|GetCurrentHP) 0.0)
        (if (>= (Variables|Default|GetLevel) 4)
          (Utilities|FlowControl|DoOnce false
            (:Completed
              (Variables|Default|SetUltSkillCondition true)
              (if (Utilities|Time|IsValidTimerHandle (Variables|Default|GetActiveSkillTimer))
                (Animation|StopAnimMontage (Variables|Default|GetActiveSkillMontage))
                (CallFunction|OnActiveSkillEnd이벤트))))
          (else
            (Default|CallCharDead)
            (Variables|Default|SetIsDead true)))))))

(fn ConstructionScript
  (|CallParentFunction))

(fn GetNearAlies
  (for _array_element (CallFunction|GetAllAliveAllies)
    (if (<= (CallFunction|GetDistancewithTarget _array_element) 7.5e+02)
      (Utilities|Array|Add (LocalVariables|GetNearCharacter) _array_element)))
  (return (LocalVariables|GetNearCharacter)))