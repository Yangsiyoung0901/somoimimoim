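; Blueprint for the Skull Collector, a combat character built around Karma debuff stacks, with level-gated passive and ultimate.
; From level 3 it puts Karma on its attackers, adding a random debuff at level 5, and its base attack scales with the target's Karma.
; Its active skill spawns at the farthest eligible enemy's direction.
; From level 4, heavy HP loss triggers a one-time death-preventing immunity and ultimate, spawned on the most Karma-stacked enemy.
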(event Custom|UnderAttackTriggered_이벤트
  (params (DamageDealer :type AI%20Character%20Base%20Object%20Reference) (Damage :type Float%20%28double-precision%29) (IsTrueDamage :type Boolean) (Target :type Boolean) (Tag :type Name))
  (if (>= (Variables|Default|GetLevel) 5)
    (Default|AddDebuffStack DamageDealer "NewEnumerator5" 2)
    (Default|AddDebuffStack DamageDealer (.OutItem (Utilities|Array|Random (Variables|Default|GetRandomDebuffs))) 2)
    (else
      (Default|AddDebuffStack DamageDealer "NewEnumerator5" 1))))

(event EventBeginPlay
  (|CallParentFunction) ; 지금 이 노드는 비활성 상태입니다. \n핀을 끌어서 다른 노드를 연결하면 활성화됩니다.
)

(event Collision|EventActorBeginOverlap
  (params (OtherActor :type Actor%20Object%20Reference))
  (|CallParentFunction OtherActor) ; 지금 이 노드는 비활성 상태입니다. \n핀을 끌어서 다른 노드를 연결하면 활성화됩니다.
)

(event EventTick
  (params (DeltaSeconds :type Float%20%28single-precision%29))
  (|CallParentFunction DeltaSeconds) ; 지금 이 노드는 비활성 상태입니다. \n핀을 끌어서 다른 노드를 연결하면 활성화됩니다.
)

(event EventBaseAttack
  (bind _attacktarget (Variables|Default|GetAttackTarget)
    (:then
      (Default|DealDamageNormal (Variables|Default|GetAttackTarget) self (+ (* (Math|Conversions|ToFloat(Integer) (Default|GetDebuffStack _attacktarget "NewEnumerator5")) 0.2) 1.0) false true "BaseAttack"))
    (:else)))

(event EventBattleStartServer
  (|CallParentFunction)
  (if (>= (Variables|Default|GetLevel) 3)
    (EventDispatchers|AssignUnderAttackTriggered (delegate Custom|UnderAttackTriggered_이벤트))
    (else
      (EventDispatchers|UnbindEventfromUnderAttackTriggered (delegate Custom|UnderAttackTriggered_이벤트)))))

(event EventLevelChange
  (params (Level :type Integer))
  (|CallParentFunction Level)
  (if (>= (Variables|Default|GetLevel) 3)
    (EventDispatchers|AssignUnderAttackTriggered (delegate Custom|UnderAttackTriggered_이벤트))
    (else
      (EventDispatchers|UnbindEventfromUnderAttackTriggered (delegate Custom|UnderAttackTriggered_이벤트)))))

(event EventApplyDamage
  (params (Damage :type Float%20%28double-precision%29) (Tag :type Name :default "None") (DamageDealer :type AI%20Character%20Base%20Object%20Reference) (IsTrueDamage :type Boolean) (IsTarget :type Boolean))
  (Default|CallApplyDamageTriggered Damage Tag DamageDealer IsTrueDamage IsTarget)
  (if (not (Variables|Default|GetIgnoreDamage))
    (bind _output_get (Variables|Default|SetCurrentHP (- (Variables|Default|GetCurrentHP) Damage)))
    (if (Math|Boolean|ANDBoolean (>= (.Percentage (CallFunction|GetLostHP)) 7e+01) (>= (Variables|Default|GetLevel) 4) (not (Variables|Default|GetUltUsed)))
      (if (<= (Variables|Default|GetCurrentHP) 0.0)
        (Variables|Default|SetCurrentHP 1.0))
      (Variables|Default|SetUltSkillCondition true)
      (Variables|Default|SetIsImmune true)
      (Variables|Default|SetIsUnstoppable true)
      (Variables|Default|SetUltUsed true)
      (Default|RemoveAllCCs (Variables|Default|GetBPC_CCs) self)
      (elif (<= _output_get 0.0)
        (Default|CallCallDangerOfDeath self)
        (Utilities|FlowControl|DelayUntilNextTick)
        (if (<= (Variables|Default|GetCurrentHP) 0.0)
          (Default|CallCharDead self)
          (Variables|Default|SetIsDead true)
          (Actor|Tick|SetActorTickEnabled false))))))

(event EventActiveSkill
  (bind _returnvalue (Transformation|GetActorLocation))
  (bind _farthesttarget (CallFunction|GetFarthestEnemy))
  (Utilities|IsValid _farthesttarget
    (:Is%20Valid
      (Game|SpawnActorfromClass "/Game/Blueprints/Characters/TheSkullCollector/BP_SkullCollector_ActiveSkill.BP_SkullCollector_ActiveSkill_C" (Math|Transform|MakeTransform _returnvalue (Math|Rotator|FindLookatRotation _returnvalue (Transformation|GetActorLocation _farthesttarget)) "1.000000,1.000000,1.000000") "Undefined" "MultiplyWithRoot" 0 _farthesttarget self 0))))

(event EventUltSkill
  (bind _targetenemy (CallFunction|GetMostKarmaStackEnemy))
  (Game|SpawnActorfromClass "/Game/Blueprints/Characters/TheSkullCollector/BP_SkullCollector_UltSkill.BP_SkullCollector_UltSkill_C" (Math|Transform|MakeTransform (- (Transformation|GetActorLocation _targetenemy) "0.000000,0.000000,60.000000") "0, 0, 0" "1.000000,1.000000,1.000000") "AlwaysSpawn" "MultiplyWithRoot" 0 (Default|GetDebuffStack _targetenemy "NewEnumerator5") self 0)
  (Utilities|FlowControl|Delay 2.0)
  (Variables|Default|SetIsImmune false)
  (Variables|Default|SetIsUnstoppable false)
  (Variables|Default|SetUltSkillCondition false))

(fn ConstructionScript
  (|CallParentFunction))

(fn GetFarthestEnemy
  (bind _returnvalue (Transformation|GetActorLocation))
  (LocalVariables|SetFarthestLocation (Transformation|GetActorLocation))
  (for _array_element (CallFunction|GetAllAliveEnemy)
    (if (and (>= (Math|Vector|Distance(Vector) _returnvalue (Transformation|GetActorLocation _array_element)) (Math|Vector|Distance(Vector) _returnvalue (LocalVariables|GetFarthestLocation))) (not (Utilities|Array|ContainsItem (Variables|/Game/BT/AICharacterBase.AICharacterBase_C|GetCCs _array_element) "NewEnumerator8")))
      (LocalVariables|SetFarthestLocation (Transformation|GetActorLocation _array_element))
      (LocalVariables|SetTempTarget _array_element)))
  (return (LocalVariables|GetTempTarget)))

(fn GetMostKarmaStackEnemy
  (for _array_element (CallFunction|GetAllAliveEnemy)
    (if (>= (Default|GetDebuffStack _array_element "NewEnumerator5") (LocalVariables|GetKarmaStack))
      (LocalVariables|SetMostStackedEnemy _array_element)
      (LocalVariables|SetKarmaStack (Default|GetDebuffStack _array_element "NewEnumerator5"))))
  (return (LocalVariables|GetMostStackedEnemy)))