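; Homing projectile for the Skull Collector's active skill that damages its target and drags it in front of the caster.
; The server steers it toward the target each tick, destroying it if the target is lost.
; A hit on the target's Hitbox deals damage scaled by debuff stacks.
; Unless the target already has the first crowd control, it applies two CCs, turns the caster, and timeline-lerps the target to a navmesh-projected point.
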(event OnComponentBeginOverlap(Sphere)
  (params (OverlappedComponent :type Primitive%20Component%20Object%20Reference) (OtherActor :type Actor%20Object%20Reference) (OtherComp :type Primitive%20Component%20Object%20Reference) (OtherBodyIndex :type Integer) (bFromSweep :type Boolean) (SweepResult :type Hit%20Result%20Structure%20%28by%20ref%29))
  (bind _spawnedcharacter (Variables|Default|GetSpawnedCharacter))
  (bind _target (Variables|Default|GetTarget))
  (bind _target_2 (Variables|Default|GetTarget))
  (bind _target_3 (Variables|Default|GetTarget))
  (bind _target_4 (Variables|Default|GetTarget))
  (bind _returnvalue (Transformation|GetActorLocation _target))
  (if (Networking|IsServer)
    (if (and (== OtherActor _target_4) (== OtherComp (Variables|/Game/BT/AICharacterBase.AICharacterBase_C|GetHitbox _target_4)))
      (Utilities|FlowControl|DoOnce false
        (:Completed
          (Default|DealDamageNormal _target_3 (Variables|Default|GetSpawnedCharacter) (* (+ (* (Math|Conversions|ToFloat(Integer) (Default|GetDebuffStack _target_4 "NewEnumerator5")) 0.2) 1.0) 2.0) false true "None")
          (if (Utilities|Array|ContainsItem (Variables|/Game/BT/AICharacterBase.AICharacterBase_C|GetCCs _target_3) "NewEnumerator8")
            (Actor|DestroyActor)
            (else
              (Default|ApplyCC (Variables|/Game/BT/AICharacterBase.AICharacterBase_C|GetBPC_CCs _target_2) "NewEnumerator8" 0.5)
              (Transformation|SetActorRotation (Variables|Default|GetSpawnedCharacter) (Math|Conversions|RotationFromXVector (Math|Vector|Normalize (- (Transformation|GetActorLocation (Variables|Default|GetTarget)) (Transformation|GetActorLocation (Variables|Default|GetSpawnedCharacter))))))
              (Default|ApplyCC (Variables|/Game/BT/AICharacterBase.AICharacterBase_C|GetBPC_CCs _target_2) "NewEnumerator2" 2.0 (Variables|Default|GetSpawnedCharacter))
              (Variables|Default|SetPullLocation (.ProjectedLocation (AI|Navigation|ProjectPointtoNavigation (+ (* (Transformation|GetActorForwardVector _spawnedcharacter) 1.5e+02) (Transformation|GetActorLocation _spawnedcharacter)) 0 0 "150.000000,150.000000,150.000000")))
              (Default|SetCharUnblocked (Variables|Default|GetTarget) true)
              (bind _새_트랙_0 (Timeline|타임라인 PlayFromStart)
                (:Update
                  (Transformation|SetActorLocation (Variables|Default|GetTarget) (Math|Vector|Lerp(Vector) _returnvalue (Math|Vector|MakeVector (.x (Variables|Default|GetPullLocation)) (.y (Variables|Default|GetPullLocation)) (.Z (Math|Vector|BreakVector _returnvalue))) _새_트랙_0) true false))
                (:Finished
                  (Default|SetCharUnblocked (Variables|Default|GetTarget) false)
                  (Actor|DestroyActor))))))))))

(event EventBeginPlay
  (|CallParentFunction) ; 지금 이 노드는 비활성 상태입니다. \n핀을 끌어서 다른 노드를 연결하면 활성화됩니다.
)

(event Collision|EventActorBeginOverlap
  (params (OtherActor :type Actor%20Object%20Reference))
  (|CallParentFunction OtherActor) ; 지금 이 노드는 비활성 상태입니다. \n핀을 끌어서 다른 노드를 연결하면 활성화됩니다.
)

(event EventTick
  (params (DeltaSeconds :type Float%20%28single-precision%29))
  (bind _returnvalue (Transformation|GetActorLocation))
  (bind _target (Variables|Default|GetTarget))
  (bind _returnvalue_2 (Transformation|GetActorLocation _target))
  (|CallParentFunction DeltaSeconds)
  (if (Networking|IsServer)
    (Utilities|IsValid _target
      (:Is%20Valid
        (Variables|/Script/Engine.MovementComponent|SetVelocity (Variables|Default|GetProjectileMovement) (* (Math|Vector|Normalize (- _returnvalue_2 _returnvalue)) 3e+03))
        (Transformation|SetActorRotation (Math|Rotator|FindLookatRotation _returnvalue _returnvalue_2)))
      (:Is%20Not%20Valid
        (Actor|DestroyActor)))))

(fn ConstructionScript
  (|CallParentFunction))