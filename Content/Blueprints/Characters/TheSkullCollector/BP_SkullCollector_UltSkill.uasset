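; BP_SkullCollector_UltSkill is the spawned area-of-effect impact actor for the Skull Collector's ultimate.
; Its construction script scales the sphere radius by Stack.
; One tick after BeginPlay, it stuns and damages overlapping AI characters not on the spawning character's team.
; Damage scales with Stack and each target's stacks of a specific debuff, and the actor destroys itself after a short delay.
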(event Custom|UltImpact
  (for _array_element (Collision|GetOverlappingActors (Variables|Default|GetSphere) "/Game/BT/AICharacterBase.AICharacterBase_C" :!class /Script/Engine.PrimitiveComponent)
    (bind _asaicharacter_base (Utilities|Casting|CastToAICharacterBase _array_element))
    (if (!= (Variables|/Game/BT/AICharacterBase.AICharacterBase_C|GetTeam _asaicharacter_base) (Variables|/Game/BT/AICharacterBase.AICharacterBase_C|GetTeam (Variables|Default|GetSpawnedCharacter)))
      (Default|Stun (Variables|/Game/BT/AICharacterBase.AICharacterBase_C|GetBPC_CCs _asaicharacter_base) 2.0)
      (Default|DealDamageNormal _asaicharacter_base (Variables|Default|GetSpawnedCharacter) (* (* (Math|Conversions|ToFloat(Integer) (Variables|Default|GetStack)) 0.8) (+ (* (Math|Conversions|ToFloat(Integer) (Default|GetDebuffStack _asaicharacter_base "NewEnumerator5")) 0.2) 1.0)) false false "None")))
  (Utilities|FlowControl|Delay 2.0)
  (Actor|DestroyActor))

(event EventBeginPlay
  (|CallParentFunction)
  (Utilities|FlowControl|DelayUntilNextTick)
  (CallFunction|UltImpact))

(event Collision|EventActorBeginOverlap
  (params (OtherActor :type Actor%20Object%20Reference))
  (|CallParentFunction OtherActor) ; 지금 이 노드는 비활성 상태입니다. \n핀을 끌어서 다른 노드를 연결하면 활성화됩니다.
)

(event EventTick
  (params (DeltaSeconds :type Float%20%28single-precision%29))
  (|CallParentFunction DeltaSeconds) ; 지금 이 노드는 비활성 상태입니다. \n핀을 끌어서 다른 노드를 연결하면 활성화됩니다.
)

(fn ConstructionScript
  (|CallParentFunction)
  (Components|Sphere|SetSphereRadius (Variables|Default|GetSphere) (Math|Conversions|ToFloat(Integer) (* (Variables|Default|GetStack) 100)) true))