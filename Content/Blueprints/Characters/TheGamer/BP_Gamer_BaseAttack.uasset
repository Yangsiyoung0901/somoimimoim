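; Base attack actor for the Gamer character that explodes on hitting an enemy's hitbox or the floor.
; On the server, either overlap plays an explosion effect, damages every living enemy AICharacterBase within Range, then destroys the actor.
; Damage is credited to SelfChar, with a higher skill multiplier when Upgraded.
; A helper that looks up an attached Ruler hidden-passive actor is defined but not called here.
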(event OnComponentBeginOverlap(Collision)
  (params (OverlappedComponent :type Primitive%20Component%20Object%20Reference) (OtherActor :type Actor%20Object%20Reference) (OtherComp :type Primitive%20Component%20Object%20Reference) (OtherBodyIndex :type Integer) (bFromSweep :type Boolean) (SweepResult :type Hit%20Result%20Structure%20%28by%20ref%29))
  (if (Networking|IsServer)
    (bind _asaicharacter_base (Utilities|Casting|CastToAICharacterBase OtherActor))
    (if (Math|Boolean|ANDBoolean (!= (Variables|/Game/BT/AICharacterBase.AICharacterBase_C|GetTeam _asaicharacter_base) (Variables|/Game/BT/AICharacterBase.AICharacterBase_C|GetTeam (Variables|Default|GetSelfChar))) (not (Variables|/Game/BT/AICharacterBase.AICharacterBase_C|GetIsDead _asaicharacter_base)) (== OtherComp (Variables|/Game/BT/AICharacterBase.AICharacterBase_C|GetHitbox _asaicharacter_base)))
      (CallFunction|PlayHitEffect)
      (for _array_element (Collision|GetOverlappingActors (Variables|Default|GetRange) "/Game/BT/AICharacterBase.AICharacterBase_C" :!class /Script/Engine.PrimitiveComponent)
        (bind _asaicharacter_base_2 (Utilities|Casting|CastToAICharacterBase _array_element))
        (if (and (!= (Variables|/Game/BT/AICharacterBase.AICharacterBase_C|GetTeam _asaicharacter_base_2) (Variables|/Game/BT/AICharacterBase.AICharacterBase_C|GetTeam (Variables|Default|GetSelfChar))) (not (Variables|/Game/BT/AICharacterBase.AICharacterBase_C|GetIsDead _asaicharacter_base_2)))
          (Default|DealDamageNormal _asaicharacter_base_2 (Variables|Default|GetSelfChar) (Math|Float|SelectFloat 3.0 2.0 (Variables|Default|GetUpgraded)) false false "BaseAttack")))
      (Actor|DestroyActor))))

(event OnComponentBeginOverlap(FloorHit)
  (params (OverlappedComponent :type Primitive%20Component%20Object%20Reference) (OtherActor :type Actor%20Object%20Reference) (OtherComp :type Primitive%20Component%20Object%20Reference) (OtherBodyIndex :type Integer) (bFromSweep :type Boolean) (SweepResult :type Hit%20Result%20Structure%20%28by%20ref%29))
  (if (Networking|IsServer)
    (CallFunction|PlayHitEffect)
    (for _array_element (Collision|GetOverlappingActors (Variables|Default|GetRange) "/Game/BT/AICharacterBase.AICharacterBase_C" :!class /Script/Engine.PrimitiveComponent)
      (bind _asaicharacter_base (Utilities|Casting|CastToAICharacterBase _array_element))
      (if (and (!= (Variables|/Game/BT/AICharacterBase.AICharacterBase_C|GetTeam _asaicharacter_base) (Variables|/Game/BT/AICharacterBase.AICharacterBase_C|GetTeam (Variables|Default|GetSelfChar))) (not (Variables|/Game/BT/AICharacterBase.AICharacterBase_C|GetIsDead _asaicharacter_base)))
        (Default|DealDamageNormal _asaicharacter_base (Variables|Default|GetSelfChar) (Math|Float|SelectFloat 3.0 2.0 (Variables|Default|GetUpgraded)) false false "BaseAttack")))
    (Actor|DestroyActor)))

(event Custom|PlayHitEffect
  (Niagara|SpawnSystematLocation "/Game/Marketplace/Sci-Fi_Starter_VFX_Pack_Niagara/Niagara/Explosion/NS_Explosion_C4_2.NS_Explosion_C4_2" (Transformation|GetActorLocation)))

(fn ConstructionScript)

(fn TargetHasHiddenPassiveActor
  (params (Target :type AI%20Character%20Base%20Object%20Reference))
  (for _array_element (Actor|GetAttachedActors Target true false)
    (bind _asbp_ruler_hidden_passive (Utilities|Casting|CastToBP_Ruler_HiddenPassive _array_element))
    (LocalVariables|SetHasActor true)
    (LocalVariables|SetNewLocalVar _asbp_ruler_hidden_passive))
  (return (LocalVariables|GetHasActor) (LocalVariables|GetNewLocalVar)))