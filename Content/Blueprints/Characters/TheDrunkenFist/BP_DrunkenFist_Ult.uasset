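; BP_DrunkenFist_Ult is the hit actor for the Drunken Fist character's ultimate, damaging the first valid enemy it overlaps.
; On the server, HitCollision overlaps are filtered to living AI characters on a different team than SpawnedCharacter, counting only their Hitbox component.
; A valid hit deals scaled normal damage credited to SpawnedCharacter under the BaseAttack tag, then destroys the actor.
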(event OnComponentBeginOverlap(HitCollision)
  (params (OverlappedComponent :type Primitive%20Component%20Object%20Reference) (OtherActor :type Actor%20Object%20Reference) (OtherComp :type Primitive%20Component%20Object%20Reference) (OtherBodyIndex :type Integer) (bFromSweep :type Boolean) (SweepResult :type Hit%20Result%20Structure%20%28by%20ref%29))
  (if (Networking|IsServer)
    (bind _asaicharacter_base (Utilities|Casting|CastToAICharacterBase OtherActor))
    (if (Math|Boolean|ANDBoolean (!= (Variables|/Game/BT/AICharacterBase.AICharacterBase_C|GetTeam _asaicharacter_base) (Variables|/Game/BT/AICharacterBase.AICharacterBase_C|GetTeam (Variables|Default|GetSpawnedCharacter))) (not (Variables|/Game/BT/AICharacterBase.AICharacterBase_C|GetIsDead _asaicharacter_base)) (== OtherComp (Variables|/Game/BT/AICharacterBase.AICharacterBase_C|GetHitbox _asaicharacter_base)))
      (bind _output_get (Variables|Default|SetHitChar _asaicharacter_base))
      (Default|DealDamageNormal _output_get (Variables|Default|GetSpawnedCharacter) 2.0 false true "BaseAttack")
      (Actor|DestroyActor))))

(event EventBeginPlay
  (|CallParentFunction) ; 지금 이 노드는 비활성 상태입니다. \n핀을 끌어서 다른 노드를 연결하면 활성화됩니다.
)

(event Collision|EventActorBeginOverlap
  (params (OtherActor :type Actor%20Object%20Reference))
  (|CallParentFunction OtherActor) ; 지금 이 노드는 비활성 상태입니다. \n핀을 끌어서 다른 노드를 연결하면 활성화됩니다.
)

(event EventTick
  (params (DeltaSeconds :type Float%20%28single-precision%29))
  (|CallParentFunction DeltaSeconds) ; 지금 이 노드는 비활성 상태입니다. \n핀을 끌어서 다른 노드를 연결하면 활성화됩니다.
)

(fn ConstructionScript
  (|CallParentFunction))