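; Drunken Fist battle character, with basic attack, active skill, ultimate and level-gated passives.
; Active skill randomly either adds an armor-granting drunken stack or heals lost HP; three stacks unlock the ultimate.
; Ultimate grants immunity and unstoppability while a looping timer sprays randomly rotated projectiles.
; From level 3 a timer debuffs nearby enemies; from level 5 the same spray runs until death, replacing attacks and skill with another AnimBP.
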(event Custom|Passive
  (if (not (Variables|Default|GetIsDead))
    (bind _nearenemies (CallFunction|GetEnemyinDistance 5e+02))
    (for _array_element _nearenemies
      (Default|AddDebuffStack _array_element "NewEnumerator0" 1)
      (CallFunction|PlayPassiveEffect _array_element))))

(event Custom|SpawnProjectile
  (Game|SpawnActorfromClass "/Game/Blueprints/Characters/TheDrunkenFist/BP_DrunkenFist_Ult.BP_DrunkenFist_Ult_C" (Math|Transform|MakeTransform (Transformation|GetActorLocation) (Math|Rotator|MakeRotator 0.0 0.0 (.yaw (Math|Random|RandomRotator false))) "1.000000,1.000000,1.000000") "Undefined" "MultiplyWithRoot" 0 self 0)
  (Game|SpawnActorfromClass "/Game/Blueprints/Characters/TheDrunkenFist/BP_DrunkenFist_Ult.BP_DrunkenFist_Ult_C" (Math|Transform|MakeTransform (Transformation|GetActorLocation) (Math|Rotator|MakeRotator 0.0 0.0 (.yaw (Math|Random|RandomRotator false))) "1.000000,1.000000,1.000000") "Undefined" "MultiplyWithRoot" 0 self 0))

(event Custom|OnUltEnd_이벤트
  (EventDispatchers|UnbindEventfromOnUltEnd (delegate Custom|OnUltEnd_이벤트))
  (Utilities|Time|ClearandInvalidateTimerbyHandle (Variables|Default|GetUltTimer))
  (Variables|Default|SetIsUnstoppable false)
  (Variables|Default|SetIsImmune false))

(event Custom|CustomEvent
  (params (Character :type AI%20Character%20Base%20Object%20Reference))
  (Utilities|Array|RemoveItem (Variables|Default|GetCCs) "NewEnumerator1")
  (Utilities|Time|ClearandInvalidateTimerbyHandle (Variables|Default|GetHiddenPassiveTimer)))

(event Custom|PlayPassiveEffect
  (params (Target :type AI%20Character%20Base%20Object%20Reference))
  (Niagara|SpawnSystemAttached "/Game/Marketplace/CharacterAuras/Effects/NS_Love_aura.NS_Love_aura" (Variables|/Script/Engine.Character|GetMesh Target) "None" "0, 0, 0" "0, 0, 0" "SnapToTarget" true))

(event EventBeginPlay
  (|CallParentFunction) ; 지금 이 노드는 비활성 상태입니다. \n핀을 끌어서 다른 노드를 연결하면 활성화됩니다.
)

(event Collision|EventActorBeginOverlap
  (params (OtherActor :type Actor%20Object%20Reference))
  (|CallParentFunction OtherActor) ; 지금 이 노드는 비활성 상태입니다. \n핀을 끌어서 다른 노드를 연결하면 활성화됩니다.
)

(event EventTick
  (params (DeltaSeconds :type Float%20%28single-precision%29))
  (|CallParentFunction DeltaSeconds) ; 지금 이 노드는 비활성 상태입니다. \n핀을 끌어서 다른 노드를 연결하면 활성화됩니다.
)

(event EventBaseAttack
  (bind _attacktarget (Variables|Default|GetAttackTarget)
    (:then
      (Default|DealDamageNormal _attacktarget self 1.0 false true "BaseAttack"))
    (:else)))

(event EventBattleStartServer
  (bind _mesh (Variables|Character|GetMesh))
  (|CallParentFunction)
  (Utilities|FlowControl|Sequence
    (:then_0
      (if (>= (Variables|Default|GetLevel) 3)
        (if (not (Utilities|Time|IsValidTimerHandle (Variables|Default|GetPassiveTimer)))
          (bind _returnvalue (Utilities|Time|SetTimerbyEvent (delegate Custom|Passive) 2.0 true))
          (Variables|Default|SetPassiveTimer _returnvalue))
        (else
          (Utilities|Time|ClearandInvalidateTimerbyHandle (Variables|Default|GetPassiveTimer)))))
    (:then_1
      (if (>= (Variables|Default|GetLevel) 5)
        (Class|SkeletalMeshComponent|SetAnimClass _mesh "/Game/Animation/AnimBlueprint/ABP_AI_DrunkenFist_HiddenPassive.ABP_AI_DrunkenFist_HiddenPassive_C")
        (bind _returnvalue_2 (Utilities|Time|SetTimerbyEvent (delegate Custom|SpawnProjectile) 0.05 true))
        (Variables|Default|SetHiddenPassiveTimer _returnvalue_2)
        (Variables|Default|SetbCanUseSkill false)
        (Variables|Default|SetbCanBaseAttack false)
        (EventDispatchers|AssignCharDead (delegate Custom|CustomEvent))
        (else
          (Class|SkeletalMeshComponent|SetAnimClass _mesh "/Game/Animation/AnimBlueprint/ABP_AI_DrunkenFist.ABP_AI_DrunkenFist_C")
          (Variables|Default|SetbCanUseSkill true)
          (Variables|Default|SetbCanBaseAttack true)
          (Utilities|Time|ClearandInvalidateTimerbyHandle (Variables|Default|GetHiddenPassiveTimer)))))))

(event EventActiveSkill
  (if (Math|Random|RandomBool)
    (CallFunction|ChangeDrunkenStack (+ (Variables|Default|GetDrunkenStack) 1))
    (CallFunction|ChangeBuffDebuffWidget "NewEnumerator6" (Variables|Default|GetDrunkenStack))
    (if (>= (Variables|Default|GetDrunkenStack) 3)
      (Utilities|FlowControl|DoOnce false
        (:Completed
          (Variables|Default|SetUltSkillCondition true))))
    (else
      (CallFunction|HealCharacter (* (* (.LostHP (CallFunction|GetLostHP)) 0.2) (Variables|Default|GetHealEffectBuff))))))

(event EventLevelChange
  (params (Level :type Integer))
  (bind _mesh (Variables|Character|GetMesh))
  (|CallParentFunction Level)
  (Utilities|FlowControl|Sequence
    (:then_0
      (if (>= (Variables|Default|GetLevel) 3)
        (if (not (Utilities|Time|IsValidTimerHandle (Variables|Default|GetPassiveTimer)))
          (bind _returnvalue (Utilities|Time|SetTimerbyEvent (delegate Custom|Passive) 2.0 true))
          (Variables|Default|SetPassiveTimer _returnvalue))
        (else
          (Utilities|Time|ClearandInvalidateTimerbyHandle (Variables|Default|GetPassiveTimer)))))
    (:then_1
      (if (>= (Variables|Default|GetLevel) 5)
        (Class|SkeletalMeshComponent|SetAnimClass _mesh "/Game/Animation/AnimBlueprint/ABP_AI_DrunkenFist_HiddenPassive.ABP_AI_DrunkenFist_HiddenPassive_C")
        (bind _returnvalue_2 (Utilities|Time|SetTimerbyEvent (delegate Custom|SpawnProjectile) 0.05 true))
        (Variables|Default|SetHiddenPassiveTimer _returnvalue_2)
        (Variables|Default|SetbCanUseSkill false)
        (Variables|Default|SetbCanBaseAttack false)
        (EventDispatchers|AssignCharDead (delegate Custom|CustomEvent))
        (else
          (Class|SkeletalMeshComponent|SetAnimClass _mesh "/Game/Animation/AnimBlueprint/ABP_AI_DrunkenFist.ABP_AI_DrunkenFist_C")
          (Variables|Default|SetbCanUseSkill true)
          (Variables|Default|SetbCanBaseAttack true)
          (Utilities|Time|ClearandInvalidateTimerbyHandle (Variables|Default|GetHiddenPassiveTimer)))))))

(event EventUltSkill
  (Variables|Default|SetUltSkillCondition false)
  (Variables|Default|SetIsUnstoppable true)
  (Variables|Default|SetIsImmune true)
  (bind _returnvalue (Utilities|Time|SetTimerbyEvent (delegate Custom|SpawnProjectile) 0.05 true))
  (Variables|Default|SetUltTimer _returnvalue)
  (EventDispatchers|AssignOnUltEnd (delegate Custom|OnUltEnd_이벤트)))

(fn ConstructionScript
  (|CallParentFunction))

(fn ChangeDrunkenStack
  (params (DrunkenStack :type Integer))
  (Variables|Default|SetBuffedArmor (- (Variables|Default|GetBuffedArmor) (* (Math|Conversions|ToFloat(Integer) (Variables|Default|GetDrunkenStack)) 2e+01)))
  (bind _output_get (Variables|Default|SetDrunkenStack DrunkenStack))
  (Variables|Default|SetBuffedArmor (+ (Variables|Default|GetBuffedArmor) (* (Math|Conversions|ToFloat(Integer) _output_get) 2e+01))))