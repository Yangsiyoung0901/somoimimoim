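; AI warrior character that hunts the nearest BP_Character_Archer, closing distance with a dash and striking it in melee.
; A looping timer retargets, starts AIMoveTo chasing and sets InRange by comparing distance to the sphere radius.
; Tick triggers cooldown-gated attacks when in range and dashes when far, briefly boosting movement speed with a fire effect.
; Attacks stop movement, play a slash effect, subtract target HP directly and call Die at zero.
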(event Custom|DealDamage
  (bind _target (Variables|Default|GetTarget))
  (Components|Activation|Activate (Variables|Default|GetNS_Fire_Slash) false)
  (Variables|Default|SetAttackCool false)
  (bind _output_get (Variables|/Game/TestMap/Blueprints/BP_Character_Archer.BP_Character_Archer_C|SetHP _target (- (Variables|/Game/TestMap/Blueprints/BP_Character_Archer.BP_Character_Archer_C|GetHP _target) 8e+01)))
  (if (<= _output_get 0.0)
    (Default|Die (Variables|Default|GetTarget)))
  (Utilities|FlowControl|Delay 0.75)
  (Variables|Default|SetAttackCool true))

(event Custom|Attack
  (Components|Movement|StopMovementImmediately (Variables|Character|GetCharacterMovement))
  (CallFunction|DealDamage)
  (Variables|Default|SetIsPlayingAnimation true)
  (Utilities|FlowControl|RetriggerableDelay 0.25)
  (Variables|Default|SetIsPlayingAnimation false))

(event Custom|Die
  (Actor|DestroyActor))

(event Custom|FindEnemy
  (bind _outactors (Actor|GetAllActorsOfClass "/Game/TestMap/Blueprints/BP_Character_Archer.BP_Character_Archer_C"))
  (bind _asbp_character_archer (Utilities|Casting|CastToBP_Character_Archer (.ReturnValue (Actor|FindNearestActor (Transformation|GetActorLocation) _outactors)))
    (:then
      (Variables|Default|SetTarget _asbp_character_archer)
      (CallFunction|ChaseEnemy)
      (if (<= (.Distance (Actor|FindNearestActor (Transformation|GetActorLocation) _outactors)) (Variables|Default|GetIn%20Sphere%20Radius))
        (Variables|Default|SetInRange true)
        (else
          (Variables|Default|SetInRange false :!label _label))))
    (:CastFailed
      (goto _label))))

(event Custom|Dash
  (bind _returnvalue (Transformation|GetActorTransform))
  (bind _charactermovement (Variables|Character|GetCharacterMovement))
  (bind _charactermovement_2 (Variables|Character|GetCharacterMovement))
  (Utilities|FlowControl|Sequence
    (:then_0
      (Variables|Default|SetDashCool false)
      (Utilities|FlowControl|RetriggerableDelay 3.0)
      (Variables|Default|SetDashCool true))
    (:then_1
      (Variables|Default|SetUsingSkill true)
      (Variables|/Script/Engine.CharacterMovementComponent|SetMaxWalkSpeed _charactermovement 4e+03)
      (Variables|/Script/Engine.CharacterMovementComponent|SetMaxAcceleration _charactermovement 5e+04)
      (AI|AIMoveTo self (+ (Transformation|GetActorLocation) (* (Transformation|GetActorForwardVector) 4e+02)) 0 5.0 false
        (:then
          (Niagara|SpawnSystematLocation "/Game/BlinkAndDashVFX/VFX_Niagara/NS_Dash_Fire.NS_Dash_Fire" (.location _returnvalue) (.rotation _returnvalue) "0.700000,0.700000,0.700000")
          (Utilities|FlowControl|Delay 0.2)
          (Variables|Default|SetUsingSkill false)
          (Utilities|FlowControl|Delay 0.2)
          (Variables|/Script/Engine.CharacterMovementComponent|SetMaxWalkSpeed _charactermovement_2 7.2e+02)
          (Variables|/Script/Engine.CharacterMovementComponent|SetMaxAcceleration _charactermovement_2 5e+03))))))

(event Custom|Chase%20Enemy
  (if (not (and (Variables|Default|GetIsPlayingAnimation) (Variables|Default|GetUsingSkill)))
    (AI|AIMoveTo self "0, 0, 0" (Variables|Default|GetTarget) 5.0 false)))

(event EventTick
  (params (DeltaSeconds :type Float%20%28single-precision%29))
  (|CallParentFunction DeltaSeconds)
  (if (Utilities|IsValid (Variables|Default|GetTarget))
    (Utilities|FlowControl|Sequence
      (:then_0
        (if (and (>= (Math|Vector|Distance(Vector) (Transformation|GetActorLocation (Variables|Default|GetTarget)) (Transformation|GetActorLocation)) 5e+02) (Variables|Default|GetDashCool))
          (CallFunction|Dash)))
      (:then_1
        (if (Math|Boolean|ANDBoolean (Variables|Default|GetAttackCool) (Variables|Default|GetInRange) (not (Variables|Default|GetUsingSkill)))
          (CallFunction|Attack))))))

(event EventBeginPlay
  (Utilities|Time|SetTimerbyEvent (delegate Custom|FindEnemy) 0.1 true)
  (Utilities|FlowControl|Delay 1.0)
  (Variables|Default|SetDashCool true))

(fn ConstructionScript
  (|CallParentFunction)
  (Components|Sphere|SetSphereRadius (Variables|Default|GetSphere) (Variables|Default|GetIn%20Sphere%20Radius) true))