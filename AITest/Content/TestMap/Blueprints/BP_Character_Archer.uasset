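; AI archer character that hunts the nearest Warrior, attacking from range and kiting away.
; A looping timer picks the target and chases it until in range.
; Tick triggers instant-damage attacks followed by retreat moves, plus cooldown-gated blink teleports when the target gets close, initially unlocked after a random delay.
; FindEvadeLocation samples random navmesh-projected points in a cone away from the target and keeps the farthest from the archer.
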(event Custom|DealDamage
  (bind _target (Variables|Default|GetTarget))
  (bind _returnvalue (Transformation|GetActorTransform _target))
  (Niagara|SpawnSystematLocation "/Game/Hack_And_Slash_FX/VFX_Niagara/Impacts/NS_Cyber_Slash_Impact.NS_Cyber_Slash_Impact" (.location _returnvalue) (.rotation _returnvalue) (.scale _returnvalue))
  (Variables|Default|SetAttackCool false)
  (bind _output_get (Variables|/Game/TestMap/Blueprints/BP_Character_Warrior.BP_Character_Warrior_C|SetHP _target (- (Variables|/Game/TestMap/Blueprints/BP_Character_Warrior.BP_Character_Warrior_C|GetHP _target) 75.0)))
  (if (<= _output_get 0.0)
    (Default|Die (Variables|Default|GetTarget)))
  (Utilities|FlowControl|Delay (Variables|Default|GetAttackSpeed))
  (Variables|Default|SetAttackCool true))

(event Custom|Attack
  (Components|Movement|StopMovementImmediately (Variables|Character|GetCharacterMovement))
  (CallFunction|DealDamage)
  (Utilities|FlowControl|RetriggerableDelay (Variables|Default|GetAttackAnimTime))
  (AI|AIMoveTo self (CallFunction|FindEvadeLocation 10 6e+02) 0 5.0 false))

(event Custom|Die
  (Actor|DestroyActor))

(event Custom|FindEnemy
  (bind _outactors (Actor|GetAllActorsOfClass "/Game/TestMap/Blueprints/BP_Character_Warrior.BP_Character_Warrior_C"))
  (bind _asbp_character_warrior (Utilities|Casting|CastToBP_Character_Warrior (.ReturnValue (Actor|FindNearestActor (Transformation|GetActorLocation) _outactors)))
    (:then
      (Variables|Default|SetTarget _asbp_character_warrior)
      (if (<= (.Distance (Actor|FindNearestActor (Transformation|GetActorLocation) _outactors)) 745.0)
        (Variables|Default|SetInRange true)
        (else
          (Variables|Default|SetInRange false)
          (AI|AIMoveTo self "0, 0, 0" (Variables|Default|GetTarget) 5.0 false))))
    (:CastFailed
      (Variables|Default|SetInRange false))))

(event Custom|Blink
  (bind _location (CallFunction|FindEvadeLocation 20 6e+02))
  (bind _returnvalue (Transformation|GetActorTransform))
  (bind _returnvalue_2 (Transformation|GetActorTransform))
  (Utilities|FlowControl|Sequence
    (:then_0
      (Variables|Default|SetBlinkCool false)
      (Utilities|FlowControl|RetriggerableDelay 3.0)
      (Variables|Default|SetBlinkCool true))
    (:then_1
      (Variables|Default|SetUsingSkill true)
      (Niagara|SpawnSystematLocation "/Game/BlinkAndDashVFX/VFX_Niagara/NS_Blink_Psionic.NS_Blink_Psionic" (.location _returnvalue_2) (.rotation _returnvalue_2))
      (Utilities|FlowControl|Delay 0.05)
      (Transformation|Teleport (Math|Vector|MakeVector (.x _location) (.y _location) (.z (Transformation|GetActorLocation))) "0, 0, 0")
      (Utilities|FlowControl|Delay 0.05)
      (Niagara|SpawnSystematLocation "/Game/BlinkAndDashVFX/VFX_Niagara/NS_Blink_Psionic.NS_Blink_Psionic" (.location _returnvalue) (.rotation _returnvalue))
      (Variables|Default|SetUsingSkill false))))

(event EventTick
  (params (DeltaSeconds :type Float%20%28single-precision%29))
  (|CallParentFunction DeltaSeconds)
  (Variables|Default|GetTarget
    (:then
      (Utilities|FlowControl|Sequence
        (:then_0
          (if (and (Variables|Default|GetBlinkCool) (<= (Math|Vector|Distance(Vector) (Transformation|GetActorLocation) (Transformation|GetActorLocation (Variables|Default|GetTarget))) 4e+02))
            (CallFunction|Blink)))
        (:then_1
          (if (Math|Boolean|ANDBoolean (Variables|Default|GetAttackCool) (Variables|Default|GetInRange) (not (Variables|Default|GetUsingSkill)))
            (CallFunction|Attack)))))
    (:else)))

(event EventBeginPlay
  (Utilities|Time|SetTimerbyEvent (delegate Custom|FindEnemy) 0.1 true)
  (Utilities|FlowControl|Delay (Math|Random|RandomFloatinRange 3.0 5.0))
  (Variables|Default|SetBlinkCool true))

(fn ConstructionScript
  (|CallParentFunction)
  (Components|Sphere|SetSphereRadius (Variables|Default|GetSphere) (Variables|Default|GetIn%20Sphere%20Radius) true))

(fn FindEvadeLocation
  (params (CalIntergration :type Integer) (EvadeDistance :type Float%20%28double-precision%29))
  (Utilities|IsValid (Variables|Default|GetTarget)
    (:Is%20Valid
      (for _index (range 0 CalIntergration)
        (LocalVariables|SetTempLocation (.ProjectedLocation (AI|Navigation|ProjectPointtoNavigation (+ (Transformation|GetActorLocation) (* (Math|Vector|RotateVectorAroundAxis (Math|Vector|GetUnitDirection(Vector) (Transformation|GetActorLocation (Variables|Default|GetTarget)) (Transformation|GetActorLocation)) (Math|Random|RandomFloatinRange -45.0 45.0) "0.000000,0.000000,1.000000") EvadeDistance)) 0 0 (Math|Conversions|ToVector(Float) EvadeDistance))))
        (if (> (Math|Vector|Distance(Vector) (Transformation|GetActorLocation) (LocalVariables|GetTempLocation)) (LocalVariables|GetMaximumDistance))
          (LocalVariables|SetMaximumDistance (Math|Vector|Distance(Vector) (Transformation|GetActorLocation) (LocalVariables|GetTempLocation)))
          (LocalVariables|SetMaximumLocation (LocalVariables|GetTempLocation))))
      (return (LocalVariables|GetMaximumLocation)))))